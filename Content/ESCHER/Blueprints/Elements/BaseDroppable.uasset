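; Base actor for VR objects that a hand can grab and drop, with auto-drop enabled.
; Grabbing spawns a proxy actor attached to the hand's unproxied root, which controls the main mesh at its initial offset while physics is off.
; If the hand is through a portal, the proxy teleports to match, and the pawn's proxy update list drives it.
; Dropping destroys the proxy and restores physics.
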(event `/Game/ESCHER/Blueprints/Core/Grabbable.Grab`
  (params (`Grabbed Component` :type "SceneComponent Object Reference") (Hand :type "/Game/ESCHER/Blueprints/Elements/Player/VRController Object Reference"))
  (bind _mainmesh (`self.MainMesh`))
  (bind _output_get (set `self.Grabber` Hand))
  (bind _returnvalue (`|SpawnActorFromClass` "/Game/ESCHER/Blueprints/Elements/ProxyActor.ProxyActor_C" (`KismetMathLibrary.MakeTransform` (`SceneComponent.K2_GetComponentLocation` (`self.MainMesh`))) "AlwaysSpawn" "OverrideRootScale" null null))
  (bind _output_get_2 (set `self.GrabProxy` _returnvalue))
  (`self.K2_AttachToComponent` _output_get_2 (`/Game/ESCHER/Blueprints/Elements/Player/VRController.UnproxiedRoot` _output_get) "None" "KeepWorld" "KeepWorld" "KeepWorld" false)
  (set `/Game/ESCHER/Blueprints/Elements/ProxyActor.ControlledComponent` _mainmesh _output_get_2)
  (set `/Game/ESCHER/Blueprints/Elements/ProxyActor.UseActor` false _output_get_2)
  (set `/Game/ESCHER/Blueprints/Elements/ProxyActor.AutoUpdate` false _output_get_2)
  (bind _parentproxy (`/Game/ESCHER/Blueprints/Elements/Player/VRController.ParentProxy` _output_get))
  (bind _activeportal (`/Game/ESCHER/Blueprints/Elements/ProxyActor.ActivePortal` _parentproxy))
  (`/Engine/EditorBlueprintResources/StandardMacros.IsValid` _activeportal
    (:`Is Valid`
      (`/Game/ESCHER/Blueprints/Elements/ProxyActor.Teleport` :`self` _output_get_2 :`Portal` _activeportal :`side` (`/Game/ESCHER/Blueprints/Elements/ProxyActor.PortalSide` _parentproxy)))
    (:`Is Not Valid`
      _))
  (set `/Game/ESCHER/Blueprints/Elements/ProxyActor.InitialOffset` (`KismetMathLibrary.ComposeTransforms` (`SceneComponent.K2_GetComponentToWorld` _mainmesh) (`KismetMathLibrary.InvertTransform` (`/Game/ESCHER/Blueprints/Elements/ProxyActor.ProxyTransform` _output_get_2))) _output_get_2)
  (`PrimitiveComponent.SetSimulatePhysics` _mainmesh false)
  (`BlueprintSetLibrary.Set_Add` (`/Game/ESCHER/Blueprints/Elements/Player/VRPawn.UpdatingProxies` (`/Game/ESCHER/Blueprints/Elements/Player/VRController.VRPawn` _output_get)) (`self.GrabProxy`)))

(event `/Game/ESCHER/Blueprints/Core/Grabbable.Drop`
  (params (`Dropped Component` :type "SceneComponent Object Reference"))
  (`BlueprintSetLibrary.Set_Remove` (`/Game/ESCHER/Blueprints/Elements/Player/VRPawn.UpdatingProxies` (`/Game/ESCHER/Blueprints/Elements/Player/VRController.VRPawn` (`self.Grabber`))) (`self.GrabProxy`))
  (set `self.Grabber` null)
  (`self.K2_DestroyActor` (`self.GrabProxy`))
  (`PrimitiveComponent.SetSimulatePhysics` (`self.MainMesh`) true))

(fn `GetGrabber`
  (params (Component :type "SceneComponent Object Reference"))
  (returns (Hand :type "/Game/ESCHER/Blueprints/Elements/Player/VRController Object Reference"))
  (return (`self.Grabber`)))

(fn `GetGrabProxy`
  (returns (Proxy :type "/Game/ESCHER/Blueprints/Elements/ProxyActor Object Reference"))
  (return (`self.GrabProxy`)))

(fn `IsAutoDropping`
  (params (Component :type "SceneComponent Object Reference"))
  (returns (AutoDrop :type Boolean))
  (return true))

(fn `IsGrabbable`
  (params (Component :type "SceneComponent Object Reference"))
  (returns (Grabbable :type Boolean))
  (return true))

(fn `UserConstructionScript`
  (`parent.UserConstructionScript`))