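; LevelVarHandler is a level helper actor that places VR players at the start and hands out ray IDs.
; On BeginPlay it collects all VRPawns, waits briefly, then teleports each to the InitialCheckpoint's location and up vector if that checkpoint is valid.
; IncrementRayID bumps a shared RayIDCount counter and returns it.
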(event `self.ReceiveBeginPlay`
  (bind _initialcheckpoint (`self.InitialCheckpoint`))
  (bind _outactors (`GameplayStatics.GetAllActorsOfClass` "/Game/ESCHER/Blueprints/Elements/VRPawn.VRPawn_C"))
  (set `self.Players` _outactors)
  (`KismetSystemLibrary.Delay` 0.1)
  (`/Engine/EditorBlueprintResources/StandardMacros.IsValid` (`self.InitialCheckpoint`)
    (:`Is Valid`
      (for _array_element (`self.Players`)
        (`/Game/ESCHER/Blueprints/Elements/VRPawn.VRTeleportTo` _array_element null (`self.K2_GetActorLocation` _initialcheckpoint) (`self.GetActorUpVector` _initialcheckpoint) (0.0 0.0 0.0) true)))))

(fn `IncrementRayID`
  (returns (ID :type Integer))
  (bind _result (`/Engine/EditorBlueprintResources/StandardMacros.IncrementInt` (`self.RayIDCount`))
    (:`  `
      (return _result))))

(fn `UserConstructionScript`)