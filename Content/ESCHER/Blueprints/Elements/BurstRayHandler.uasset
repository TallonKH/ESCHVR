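; BurstRayHandler fires instant trace-based burst rays, split into segments that carry depth, accumulated distance and a unique ID from LevelVarHandler.
; PrimaryFire starts a segment at max distance, then broadcasts the collected segment IDs.
; SegmentFire walks multi-trace hits, skipping ignored components and letting BurstRayDetecting actors decide effects, termination and whether overlaps block.
; Event dispatchers report each pass, block and fired segment.
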(event `self.ReceiveBeginPlay`
  (bind _outactors (`GameplayStatics.GetAllActorsOfClass` "/Game/ESCHER/Blueprints/Elements/LevelVarHandler.LevelVarHandler_C"))
  (set `self.LevelVarHandler` (`|GetArrayItem` _outactors)))

(event `self.ReceiveDestroyed`)

(fn `PrimaryFire`
  (params (From :type "Vector Structure") (Towards :type "Vector Structure"))
  (`self.SegmentFire` From Towards (`self.MaxDistance`) 0 0.0 (`|MakeSet`))
  (`self.PrimaryFinished` self (`self.CurrentSegmentIDs`))
  (set `self.CurrentSegmentIDs` (`|MakeArray`)))

(fn `SegmentFire`
  (params (From :type "Vector Structure") (Towards :type "Vector Structure") (Distance :type "Float (double-precision)") (Depth :type Integer) (AccumulatedDistance :type "Float (double-precision)") (SegmentComponentsToIgnore :type "Set of PrimitiveComponent Object Reference (by ref)"))
  (locals (CurrentHit :type "HitResult Structure") (CurrentSegmentInfo :type "/Game/ESCHER/Blueprints/Core/BurstRaySegmentInfo Structure") (LocalEnd :type "Vector Structure"))
  (bind _currenthit (`local.CurrentHit`))
  (bind _currentsegmentinfo (`local.CurrentSegmentInfo`))
  (`|ExecutionSequence`
    (:`then_0`
      (bind _id (`/Game/ESCHER/Blueprints/Elements/LevelVarHandler.IncrementRayID` (`self.LevelVarHandler`)))
      (bind _output_get (set `self.EndLocation` (+ From (* Towards Distance))))
      (bind _output_get_2 (set `local.LocalEnd` _output_get))
      (bind _burstraysegmentinfo (make `/Game/ESCHER/Blueprints/Core/BurstRaySegmentInfo` Depth AccumulatedDistance Towards From _id))
      (set `local.CurrentSegmentInfo` _burstraysegmentinfo)
      (`KismetArrayLibrary.Array_Add` (`self.CurrentSegmentIDs`) (`.UniqueID_15_71EF2DF648B9DCD6FBC453A93F241C8E` (break `/Game/ESCHER/Blueprints/Core/BurstRaySegmentInfo` _burstraysegmentinfo)))
      (bind _outhits (`KismetSystemLibrary.LineTraceMulti` From _output_get_2 (`self.TraceChannel`) false (`self.ActorsToIgnore`)))
      (for _array_element _outhits
        (bind _output_get_3 (set `local.CurrentHit` _array_element))
        (bind (_bblockinghit _binitialoverlap _time _distance _location _impactpoint _normal _impactnormal _physmat _hitactor _hitcomponent) (`GameplayStatics.BreakHitResult` _output_get_3))
        (if (or (`BlueprintSetLibrary.Set_Contains` (`self.ComponentsToIgnore`) _hitcomponent) (`BlueprintSetLibrary.Set_Contains` SegmentComponentsToIgnore _hitcomponent))
          _
          (elif _bblockinghit
            (`|ExecutionSequence`
              (:`then_0`
                (bind _output_get_4 (set `self.EndLocation` _location))
                (set `local.LocalEnd` _output_get_4)
                (set `self.EndHit` (`local.CurrentHit`))
                (set `self.BlockedTerminally` true))
              (:`then_1`
                (bind _asburst_ray_detecting (cast `/Game/ESCHER/Blueprints/Core/BurstRayDetecting` _hitactor)
                  (:`then`
                    (bind (_doeffects _terminal) (`/Game/ESCHER/Blueprints/Core/BurstRayDetecting.BlockedBRay` _asburst_ray_detecting self (`local.CurrentSegmentInfo`) (`local.CurrentHit`)))
                    (`self.RayBlocked` self (`local.CurrentSegmentInfo`) (`local.CurrentHit`) _doeffects _terminal))
                  (:`CastFailed`
                    (`self.RayBlocked` self (`local.CurrentSegmentInfo`) (`local.CurrentHit`) true true))))
              (:`then_2`
                (break)))
            (else
              (bind _asburst_ray_detecting_2 (cast `/Game/ESCHER/Blueprints/Core/BurstRayDetecting` _hitactor)
                (:`then`
                  (bind (_doeffects_2 _block _terminal_2) (`/Game/ESCHER/Blueprints/Core/BurstRayDetecting.PassedBRay` _asburst_ray_detecting_2 self (`local.CurrentSegmentInfo`) (`local.CurrentHit`)))
                  (if _block
                    (set `local.LocalEnd` _location)
                    (if _terminal_2
                      (set `self.EndLocation` _location)
                      (set `self.EndHit` (`local.CurrentHit`))
                      (set `self.BlockedTerminally` true))
                    (`self.RayBlocked` self _currentsegmentinfo _currenthit _doeffects_2 _terminal_2)
                    (break)
                    (else
                      (`self.RayPassed` self _currentsegmentinfo _currenthit _doeffects_2))))
                (:`CastFailed`
                  (`self.RayPassed` self _currentsegmentinfo _currenthit true))))))))
    (:`then_1`
      (`self.SegmentFired` self (`local.CurrentSegmentInfo`) From (`local.LocalEnd`)))))

(fn `UserConstructionScript`)