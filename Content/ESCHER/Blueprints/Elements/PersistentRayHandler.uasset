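; Actor that manages a persistent ray built from PersistentRaySegment objects, starting and ending it on primary fire.
; It creates a root segment with max distance, registers each segment by an ID from LevelVarHandler, and broadcasts creation.
; While active, manual or self-driven Tick updates refresh the root segment and fire a post-update event.
; It provides multi line traces and can spawn a BurstRayHandler copy from the last root source and direction.
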(event `self.ReceiveBeginPlay`
  (bind _outactors (`GameplayStatics.GetAllActorsOfClass` "/Game/ESCHER/Blueprints/Elements/LevelVarHandler.LevelVarHandler_C"))
  (bind _output_get (set `self.LevelVarHandler` (`|GetArrayItem` _outactors)))
  (bind _id (`/Game/ESCHER/Blueprints/Elements/LevelVarHandler.IncrementRayID` _output_get))
  (set `self.HandlerID` _id))

(event `ManualUpdate`
  (if (`self.RayActive`) :!label _label
    (`/Game/ESCHER/Blueprints/Elements/PersistentRaySegment.UpdatePRaySegment` (`self.RootSegment`))
    (`self.OnRayPostUpdate` self)))

(event `self.ReceiveTick`
  (params (DeltaSeconds :type "Float (single-precision)"))
  (if (`self.SelfUpdating`)
    (goto _label)))

(fn `CopyBurst`
  (returns (BurstHandler :type "/Game/ESCHER/Blueprints/Elements/BurstRayHandler Object Reference"))
  (bind _returnvalue (`|SpawnActorFromClass` "/Game/ESCHER/Blueprints/Elements/BurstRayHandler.BurstRayHandler_C" (`/Game/ESCHER/Blueprints/Core/BasicMacros.BlankTransform`) "Undefined" "OverrideRootScale" null null))
  (set `/Game/ESCHER/Blueprints/Elements/BurstRayHandler.MaxDistance` (`self.MaxDistance`) _returnvalue)
  (set `/Game/ESCHER/Blueprints/Elements/BurstRayHandler.TraceChannel` (`self.TraceChannel`) _returnvalue)
  (`/Game/ESCHER/Blueprints/Elements/BurstRayHandler.PrimaryFire` _returnvalue (`self.LastRootSourceLocation`) (`self.LastRootTowards`))
  (return _returnvalue))

(fn `CreateSegment`
  (params (Parent :type "/Game/ESCHER/Blueprints/Elements/PersistentRaySegment Object Reference"))
  (returns (Segment :type "/Game/ESCHER/Blueprints/Elements/PersistentRaySegment Object Reference"))
  (bind _id (`/Game/ESCHER/Blueprints/Elements/LevelVarHandler.IncrementRayID` (`self.LevelVarHandler`)))
  (bind _returnvalue (`|GenericCreateObject` "/Game/ESCHER/Blueprints/Elements/PersistentRaySegment.PersistentRaySegment_C" self Parent self _id))
  (`BlueprintMapLibrary.Map_Add` (`self.Segments`) (`/Game/ESCHER/Blueprints/Elements/PersistentRaySegment.SegmentID` _returnvalue) _returnvalue)
  (`/Game/ESCHER/Blueprints/Elements/PersistentRaySegment.Init` _returnvalue)
  (`self.OnSegmentCreated` self _returnvalue)
  (return _returnvalue))

(fn `DoLineTrace`
  (params (Start :type "Vector Structure") (End :type "Vector Structure") (ActorsToIgnore :type "Array of Actor Object Reference (by ref)"))
  (returns (OutHits :type "Array of HitResult Structure") (ReturnValue :type Boolean))
  (bind (_outhits _returnvalue) (`KismetSystemLibrary.LineTraceMulti` Start End (`self.TraceChannel`) false ActorsToIgnore))
  (return _outhits _returnvalue))

(fn `EndPrimaryFire`
  (if (`self.RayActive`)
    (`/Game/ESCHER/Blueprints/Elements/PersistentRaySegment.Destroy` (`self.RootSegment`))))

(fn `StartPrimaryFire`
  (if (not (`self.RayActive`))
    (set `self.RayActive` true)
    (set `self.Segments` (`|MakeMap`))
    (bind _segment (`self.CreateSegment` null))
    (set `self.RootSegment` _segment)
    (set `/Game/ESCHER/Blueprints/Elements/PersistentRaySegment.Distance` (`self.MaxDistance`) _segment)))

(fn `UserConstructionScript`)