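; VRController is a Blueprint element in ESCHER that creates and positions ghost duplicates of its Model mesh.
; CreateGhost spawns a GhostObj at a far-off location, copies the Model's mesh onto its GhostMesh and returns it.
; UpdateGhost places a given ghost by re-parenting the Model's world transform from one reference frame to another, so the copy mirrors the Model's pose relative to the target frame.
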(event `/Game/ESCHER/Blueprints/Core/Ghostable.UpdateGhost`
  (params (Ghost :type "/Game/ESCHER/Blueprints/Elements/GhostObj Object Reference") (From :type "Transform Structure") (To :type "Transform Structure"))
  (`SceneComponent.K2_SetWorldTransform` (`/Game/ESCHER/Blueprints/Elements/GhostObj.GhostMesh` Ghost) (`/Game/ESCHER/Blueprints/Core/BasicMacros.ReParentTransform` (`SceneComponent.K2_GetComponentToWorld` (`self.Model`)) From To) false false))

(fn `CreateGhost`
  (returns (Ghost :type "/Game/ESCHER/Blueprints/Elements/GhostObj Object Reference"))
  (bind _returnvalue (`|SpawnActorFromClass` "/Game/ESCHER/Blueprints/Elements/GhostObj.GhostObj_C" (`KismetMathLibrary.MakeTransform` (1000000.0 1000000.0 1000000.0)) "Undefined" "OverrideRootScale" null null))
  (`/Game/ESCHER/Blueprints/Core/BasicMacros.CopyMesh` (`self.Model`) (`/Game/ESCHER/Blueprints/Elements/GhostObj.GhostMesh` _returnvalue))
  (return _returnvalue))

(fn `UserConstructionScript`)