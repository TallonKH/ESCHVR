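; GhostCreationRegion is a portal-side volume that shows ghost copies of objects at the linked portal.
; Overlapping Ghostable actors each create a ghost, stored in an actor-to-ghost map until they leave the region or are destroyed.
; Every tick each actor updates its ghost using the two port transforms, ordered by the Side flag.
; The construction script gives the region material a random hue.
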(event `self.ReceiveBeginPlay`
  ;[1 0 0.06253] WARNING: VRPawns cannot spawn inside of ghost region on BeginPlay!
  ;
  ;  (i don't know why, fix this later)
  (for _array_element (`PrimitiveComponent.GetOverlappingActors` (`self.Region`) "/Script/Engine.Actor")
    (`self.RegisterObject` _array_element)))

(event `self.ReceiveTick`
  (params (DeltaSeconds :type "Float (single-precision)"))
  (bind _portal (`self.Portal`))
  (bind _side (`self.Side`))
  (bind _returnvalue (`SceneComponent.K2_GetComponentToWorld` (`/Game/ESCHER/Blueprints/Elements/InvisPortal.PortA` _portal)))
  (bind _returnvalue_2 (`SceneComponent.K2_GetComponentToWorld` (`/Game/ESCHER/Blueprints/Elements/InvisPortal.PortB` _portal)))
  (bind _keys (`BlueprintMapLibrary.Map_Keys` (`self.ObjGhosts`)))
  (for _array_element _keys
    (bind _asghostable (cast `/Game/ESCHER/Blueprints/Core/Ghostable` _array_element))
    (`/Game/ESCHER/Blueprints/Core/Ghostable.UpdateGhost` _asghostable (`BlueprintMapLibrary.Map_Find` (`self.ObjGhosts`) _array_element) (`KismetMathLibrary.SelectTransform` _returnvalue _returnvalue_2 _side) (`KismetMathLibrary.SelectTransform` _returnvalue_2 _returnvalue _side))))

(event `self.Region.OnComponentBeginOverlap`
  (params (OverlappedComponent :type "PrimitiveComponent Object Reference") (OtherActor :type "Actor Object Reference") (OtherComp :type "PrimitiveComponent Object Reference") (OtherBodyIndex :type Integer) (bFromSweep :type Boolean) (SweepResult :type "HitResult Structure (by ref)"))
  (`self.RegisterObject` OtherActor)
  (add `self.OnDestroyed` OtherActor (delegate `Unregister Object`)))

(event `self.Region.OnComponentEndOverlap`
  (params (OverlappedComponent :type "PrimitiveComponent Object Reference") (OtherActor :type "Actor Object Reference") (OtherComp :type "PrimitiveComponent Object Reference") (OtherBodyIndex :type Integer))
  (`self.Unregister Object` OtherActor))

(event `Unregister Object`
  (params (DestroyedActor :type "Actor Object Reference"))
  (bind (_value _returnvalue) (`BlueprintMapLibrary.Map_Find` (`self.ObjGhosts`) DestroyedActor))
  (if _returnvalue
    (`self.K2_DestroyActor` _value)
    (`BlueprintMapLibrary.Map_Remove` (`self.ObjGhosts`) DestroyedActor)
    (remove `self.OnDestroyed` DestroyedActor (delegate `Unregister Object`))))

(fn `RegisterObject`
  (params (`Ghostable Object` :type "Actor Object Reference"))
  (if (not (`.ReturnValue` (`BlueprintMapLibrary.Map_Find` (`self.ObjGhosts`) `Ghostable Object`)))
    (bind _asghostable (cast `/Game/ESCHER/Blueprints/Core/Ghostable` `Ghostable Object`))
    (bind _ghost (`/Game/ESCHER/Blueprints/Core/Ghostable.CreateGhost` _asghostable))
    (`BlueprintMapLibrary.Map_Add` (`self.ObjGhosts`) `Ghostable Object` _ghost)))

(fn `UserConstructionScript`
  (`MeshComponent.SetVectorParameterValueOnMaterials` (`self.Region`) "Color" (`KismetMathLibrary.Conv_LinearColorToVector` (`KismetMathLibrary.HSVToRGB_Vector` (make `LinearColor` (`KismetMathLibrary.RandomFloatInRange` 0.0 360.0) 0.75 1.0 1.0)))))