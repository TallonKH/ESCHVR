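; Region actor that mirrors Ghostable objects and rays inside it at each Marker actor, re-parented from its own transform to the Marker's.
; Overlapping objects get one ghost per Marker, updated every Tick and destroyed on exit.
; Rays pass unblocked; B-rays emit ghost segments when they finish or cross a side, while persistent rays update theirs to the farthest side hit.
; Known bug: VRPawns cannot spawn inside the region on BeginPlay.
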(event `self.ReceiveBeginPlay`
  ;[1 0 0.06253] WARNING: VRPawns cannot spawn inside of ghost region on BeginPlay!
  ;
  ;  (i don't know why, fix this later)
  (`|ExecutionSequence`
    (:`then_0`
      (set `self.Sides` (`|MakeArray` (`self.SideXP`) (`self.SideXN`) (`self.SideYP`) (`self.SideYN`) (`self.SideZP`) (`self.SideZN`))))
    (:`then_1`
      (for _array_element (`PrimitiveComponent.GetOverlappingActors` (`self.Region`) "/Script/Engine.Actor")
        (`self.RegisterObject` _array_element)))))

(event `self.ReceiveTick`
  (params (DeltaSeconds :type "Float (single-precision)"))
  (bind _keys (`BlueprintMapLibrary.Map_Keys` (`self.ObjGhosts`)))
  (for _array_element _keys
    (bind _asghostable (cast `/Game/ESCHER/Blueprints/Core/Ghostable` _array_element))
    (for (_array_element_2 _array_index) (`/Game/ESCHER/Blueprints/Core/GhostObjList.GhostObjs` (`BlueprintMapLibrary.Map_Find` (`self.ObjGhosts`) _array_element))
      (`/Game/ESCHER/Blueprints/Core/Ghostable.UpdateGhost` _asghostable _array_element_2 (`self.GetTransform`) (`self.GetTransform` (`|GetArrayItem` (`self.Markers`) _array_index))))))

(event `self.Region.OnComponentBeginOverlap`
  (params (OverlappedComponent :type "PrimitiveComponent Object Reference") (OtherActor :type "Actor Object Reference") (OtherComp :type "PrimitiveComponent Object Reference") (OtherBodyIndex :type Integer) (bFromSweep :type Boolean) (SweepResult :type "HitResult Structure (by ref)"))
  (`self.RegisterObject` OtherActor)
  (add `self.OnDestroyed` OtherActor (delegate `Unregister Object`)))

(event `self.Region.OnComponentEndOverlap`
  (params (OverlappedComponent :type "PrimitiveComponent Object Reference") (OtherActor :type "Actor Object Reference") (OtherComp :type "PrimitiveComponent Object Reference") (OtherBodyIndex :type Integer))
  (`self.Unregister Object` OtherActor))

(event `Unregister Object`
  (params (DestroyedActor :type "Actor Object Reference"))
  (bind (_value _returnvalue) (`BlueprintMapLibrary.Map_Find` (`self.ObjGhosts`) DestroyedActor))
  (if _returnvalue
    (for _array_element (`/Game/ESCHER/Blueprints/Core/GhostObjList.GhostObjs` _value)
      (`self.K2_DestroyActor` _array_element))
    (`BlueprintMapLibrary.Map_Remove` (`self.ObjGhosts`) DestroyedActor)
    (remove `self.OnDestroyed` DestroyedActor (delegate `Unregister Object`))))

(event `StartTrackingBRay`
  (params (Handler :type "/Game/ESCHER/Blueprints/Elements/BurstRayHandler Object Reference"))
  (add `/Game/ESCHER/Blueprints/Elements/BurstRayHandler.SegmentFired` Handler (delegate `TrackedRayFinished`))
  (add `/Game/ESCHER/Blueprints/Elements/BurstRayHandler.PrimaryFinished` Handler (delegate `TrackedBRayDone`)))

(event `TrackedBRayDone`
  (params (Handler :type "/Game/ESCHER/Blueprints/Elements/BurstRayHandler Object Reference") (SegmentIDs :type "Array of Integer (by ref)"))
  (remove `/Game/ESCHER/Blueprints/Elements/BurstRayHandler.SegmentFired` Handler (delegate `TrackedRayFinished`))
  (remove `/Game/ESCHER/Blueprints/Elements/BurstRayHandler.PrimaryFinished` Handler (delegate `TrackedBRayDone`)))

(event `TrackedRayFinished`
  (params (Handler :type "/Game/ESCHER/Blueprints/Elements/BurstRayHandler Object Reference") (SegmentInfo :type "/Game/ESCHER/Blueprints/Core/BurstRaySegmentInfo Structure") (SegmentStart :type "Vector Structure") (SegmentEnd :type "Vector Structure"))
  (bind _returnvalue (`self.GetTransform`))
  (bind (_value _returnvalue_2) (`BlueprintMapLibrary.Map_Find` (`self.EnteredBRays`) (`.UniqueID_15_71EF2DF648B9DCD6FBC453A93F241C8E` (break `/Game/ESCHER/Blueprints/Core/BurstRaySegmentInfo` SegmentInfo))))
  (if _returnvalue_2
    (for _array_element (`self.Markers`)
      (bind _returnvalue_3 (`self.GetTransform` _array_element))
      (`/Game/ESCHER/Blueprints/Elements/BurstRayHandler.GhostSegmentCreated` Handler Handler SegmentInfo (`/Game/ESCHER/Blueprints/Core/BasicMacros.ReParentPosition` _value _returnvalue _returnvalue_3) (`/Game/ESCHER/Blueprints/Core/BasicMacros.ReParentPosition` SegmentEnd _returnvalue _returnvalue_3)))))

(event `StartTrackingPRay`
  (params (Segment :type "/Game/ESCHER/Blueprints/Elements/PersistentRaySegment Object Reference"))
  (add `/Game/ESCHER/Blueprints/Elements/PersistentRaySegment.UpdatePostSelfPreChildren` Segment (delegate `TrackedPRayUpdated`)))

(event `StopTrackingPRay`
  (params (Segment :type "/Game/ESCHER/Blueprints/Elements/PersistentRaySegment Object Reference"))
  (bind _trackedprays (`self.TrackedPRays`))
  (remove `/Game/ESCHER/Blueprints/Elements/PersistentRaySegment.UpdatePostSelfPreChildren` Segment (delegate `TrackedPRayUpdated`))
  (for _array_element (`/Game/ESCHER/Blueprints/Core/GhostPSegList.GhostObjs` (`BlueprintMapLibrary.Map_Find` _trackedprays Segment))
    (`/Game/ESCHER/Blueprints/Elements/PersistentRayHandler.OnGhostSegmentDestroyed` (`/Game/ESCHER/Blueprints/Elements/PersistentRaySegment.Handler` Segment) _array_element))
  (`BlueprintMapLibrary.Map_Remove` _trackedprays Segment))

(event `TrackedPRayUpdated`
  (params (UpdatedSegment :type "/Game/ESCHER/Blueprints/Elements/PersistentRaySegment Object Reference"))
  (bind _returnvalue (`self.GetTransform`))
  (bind _lastpassedcomponents (`/Game/ESCHER/Blueprints/Elements/PersistentRaySegment.LastPassedComponents` UpdatedSegment))
  (bind (_value _returnvalue_2) (`BlueprintMapLibrary.Map_Find` (`self.TrackedPRays`) UpdatedSegment))
  (bind (_bblockinghit _binitialoverlap _time _distance _location) (`GameplayStatics.BreakHitResult` (`BlueprintMapLibrary.Map_Find` _lastpassedcomponents (`self.Region`))))
  (if _returnvalue_2
    (set `self.CurrentFarthestPSideHit` (`/Game/ESCHER/Blueprints/Elements/PersistentRaySegment.EndLocation` UpdatedSegment))
    (set `self.CurrentFarthestPSideHitDist` _distance)
    (for _array_element (`self.Sides`)
      (bind (_value_2 _returnvalue_3) (`BlueprintMapLibrary.Map_Find` _lastpassedcomponents _array_element))
      (if _returnvalue_3
        (bind (_bblockinghit_2 _binitialoverlap_2 _time_2 _distance_2 _location_2) (`GameplayStatics.BreakHitResult` _value_2))
        (if (> _distance_2 (`self.CurrentFarthestPSideHitDist`))
          (set `self.CurrentFarthestPSideHitDist` _distance_2)
          (set `self.CurrentFarthestPSideHit` _location_2))))
    (for (_array_element_2 _array_index) (`/Game/ESCHER/Blueprints/Core/GhostPSegList.GhostObjs` _value)
      (bind _returnvalue_4 (`self.GetTransform` (`|GetArrayItem` (`self.Markers`) _array_index)))
      (set `/Game/ESCHER/Blueprints/Elements/GhostPersistentRaySegment.Start` (`/Game/ESCHER/Blueprints/Core/BasicMacros.ReParentPosition` _location _returnvalue _returnvalue_4) _array_element_2)
      (set `/Game/ESCHER/Blueprints/Elements/GhostPersistentRaySegment.End` (`/Game/ESCHER/Blueprints/Core/BasicMacros.ReParentPosition` (`self.CurrentFarthestPSideHit`) _returnvalue _returnvalue_4) _array_element_2)
      (`/Game/ESCHER/Blueprints/Elements/GhostPersistentRaySegment.GhostSegUpdated` _array_element_2 _array_element_2))))

(event `/Game/ESCHER/Blueprints/Core/PersistentRayDetecting.EndedPassPRay`
  (params (UnhitComponent :type "PrimitiveComponent Object Reference") (Segment :type "/Game/ESCHER/Blueprints/Elements/PersistentRaySegment Object Reference") (Handler :type "/Game/ESCHER/Blueprints/Elements/PersistentRayHandler Object Reference"))
  (if (== UnhitComponent (`self.Region`))
    (`self.StopTrackingPRay` Segment)))

(fn `BeganBlockPRay`
  (params (Hit :type "HitResult Structure") (Segment :type "/Game/ESCHER/Blueprints/Elements/PersistentRaySegment Object Reference") (RayHandler :type "/Game/ESCHER/Blueprints/Elements/PersistentRayHandler Object Reference"))
  (returns (`Do Effects` :type Boolean) (Terminal :type Boolean))
  (return false false))

(fn `BeganPassPRay`
  (params (Hit :type "HitResult Structure") (Segment :type "/Game/ESCHER/Blueprints/Elements/PersistentRaySegment Object Reference") (RayHandler :type "/Game/ESCHER/Blueprints/Elements/PersistentRayHandler Object Reference"))
  (returns (DoEffects :type Boolean) (ShouldBlock :type Boolean) (Terminal :type Boolean))
  (if (== (`.HitComponent` (`GameplayStatics.BreakHitResult` Hit)) (`self.Region`))
    (bind _returnvalue (`|GenericCreateObject` "/Game/ESCHER/Blueprints/Core/GhostPSegList.GhostPSegList_C" self))
    (for _ (`self.Markers`)
      (bind _returnvalue_2 (`|GenericCreateObject` "/Game/ESCHER/Blueprints/Elements/GhostPersistentRaySegment.GhostPersistentRaySegment_C" self))
      (`KismetArrayLibrary.Array_Add` (`/Game/ESCHER/Blueprints/Core/GhostPSegList.GhostObjs` _returnvalue) _returnvalue_2)
      (set `/Game/ESCHER/Blueprints/Elements/GhostPersistentRaySegment.AssociatedSegment` Segment _returnvalue_2)
      (`/Game/ESCHER/Blueprints/Elements/PersistentRayHandler.OnGhostSegmentCreated` RayHandler _returnvalue_2))
    (`BlueprintMapLibrary.Map_Add` (`self.TrackedPRays`) Segment _returnvalue)
    (`self.StartTrackingPRay` Segment))
  (return false false false))

(fn `BlockedBRay`
  (params (RayHandler :type "/Game/ESCHER/Blueprints/Elements/BurstRayHandler Object Reference") (SegmentInfo :type "/Game/ESCHER/Blueprints/Core/BurstRaySegmentInfo Structure") (Hit :type "HitResult Structure"))
  (returns (DoEffects :type Boolean) (Terminal :type Boolean))
  (return false false))

(fn `IsPRPassBlocking`
  (params (Component :type "PrimitiveComponent Object Reference") (Segment :type "/Game/ESCHER/Blueprints/Elements/PersistentRaySegment Object Reference"))
  (returns (Block :type Boolean))
  (return false))

(fn `PassedBRay`
  (params (RayHandler :type "/Game/ESCHER/Blueprints/Elements/BurstRayHandler Object Reference") (SegmentInfo :type "/Game/ESCHER/Blueprints/Core/BurstRaySegmentInfo Structure") (Hit :type "HitResult Structure"))
  (returns (DoEffects :type Boolean) (Block :type Boolean) (Terminal :type Boolean))
  (bind (_depth _accumulateddistance _direction _start _uniqueid) (break `/Game/ESCHER/Blueprints/Core/BurstRaySegmentInfo` SegmentInfo))
  (bind _returnvalue (`self.GetTransform`))
  (bind (_bblockinghit _binitialoverlap _time _distance _location _impactpoint _normal _impactnormal _physmat _hitactor _hitcomponent) (`GameplayStatics.BreakHitResult` Hit))
  (bind (_value _returnvalue_2) (`BlueprintMapLibrary.Map_Find` (`self.EnteredBRays`) _uniqueid))
  (if (== _hitcomponent (`self.Region`))
    (`BlueprintMapLibrary.Map_Add` (`self.EnteredBRays`) _uniqueid _location)
    (`self.StartTrackingBRay` RayHandler)
    (return false false false)
    (elif _returnvalue_2
      (for _array_element (`self.Markers`)
        (bind _returnvalue_3 (`self.GetTransform` _array_element))
        (`/Game/ESCHER/Blueprints/Elements/BurstRayHandler.GhostSegmentCreated` RayHandler RayHandler SegmentInfo (`/Game/ESCHER/Blueprints/Core/BasicMacros.ReParentPosition` _value _returnvalue _returnvalue_3) (`/Game/ESCHER/Blueprints/Core/BasicMacros.ReParentPosition` _location _returnvalue _returnvalue_3)))
      (`BlueprintMapLibrary.Map_Remove` (`self.EnteredBRays`) _uniqueid)
      (return false false false)
      (else
        (return false false false)))))

(fn `RegisterObject`
  (params (`Ghostable Object` :type "Actor Object Reference"))
  (if (not (`.ReturnValue` (`BlueprintMapLibrary.Map_Find` (`self.ObjGhosts`) `Ghostable Object`)))
    (bind _asghostable (cast `/Game/ESCHER/Blueprints/Core/Ghostable` `Ghostable Object`))
    (bind _returnvalue (`|GenericCreateObject` "/Game/ESCHER/Blueprints/Core/GhostObjList.GhostObjList_C" self))
    (for _ (`self.Markers`)
      (bind _ghost (`/Game/ESCHER/Blueprints/Core/Ghostable.CreateGhost` _asghostable))
      (`KismetArrayLibrary.Array_Add` (`/Game/ESCHER/Blueprints/Core/GhostObjList.GhostObjs` _returnvalue) _ghost))
    (`BlueprintMapLibrary.Map_Add` (`self.ObjGhosts`) `Ghostable Object` _returnvalue)))

(fn `UserConstructionScript`
  (`MeshComponent.SetVectorParameterValueOnMaterials` (`self.Region`) "Color" (`KismetMathLibrary.Conv_LinearColorToVector` (`KismetMathLibrary.HSVToRGB_Vector` (make `LinearColor` (`KismetMathLibrary.RandomFloatInRange` 0.0 360.0) 0.75 1.0 1.0)))))