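; TestBall is a grabbable test actor whose physics mesh is launched on BeginPlay with an initial velocity given in its local space.
; Grab attaches the mesh to the hand's model, while Drop detaches it and re-enables physics simulation; it always reports itself grabbable and auto-dropping.
; Disconnected leftover nodes would spawn a BurstRayHandler, fire it along the mesh's forward vector and draw its segments as debug lines.
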(event `/Game/ESCHER/Blueprints/Core/Grabbable.Grab`
  (params (`Grabbed Component` :type "SceneComponent Object Reference") (Hand :type "/Game/ESCHER/Blueprints/Elements/VRController Object Reference"))
  (bind _output_get (set `self.Grabber` Hand))
  (`SceneComponent.K2_AttachToComponent` (`self.MainMesh`) (`/Game/ESCHER/Blueprints/Elements/VRController.Model` _output_get) "None" "KeepWorld" "KeepWorld" "KeepWorld" true))

(event `/Game/ESCHER/Blueprints/Core/Grabbable.Drop`
  (params (`Dropped Component` :type "SceneComponent Object Reference"))
  (set `self.Grabber` null)
  (`SceneComponent.K2_DetachFromComponent` (`self.MainMesh`) "KeepWorld" "KeepWorld" "KeepWorld" true)
  (`PrimitiveComponent.SetSimulatePhysics` (`self.MainMesh`) true))

(event `self.ReceiveTick`
  (params (DeltaSeconds :type "Float (single-precision)"))
  (`parent.ReceiveTick` DeltaSeconds))

(event `self.ReceiveBeginPlay`
  (`PrimitiveComponent.SetPhysicsLinearVelocity` (`self.MainMesh`) (`KismetMathLibrary.TransformDirection` (`SceneComponent.K2_GetComponentToWorld` (`self.MainMesh`)) (`self.InitialVelocity`)) false "None"))

(event `segc`
  (params (Start :type "Vector Structure") (End :type "Vector Structure") (SegmentDepth :type Integer))
  (`KismetSystemLibrary.DrawDebugLine` Start End (struct :`G` 1.0 :`B` 0.990355 :`A` 1.0) 5.0 1.0))

(event `brfin`
  (params (Handler :type "/Game/ESCHER/Blueprints/Core/BurstRayHandler Object Reference") (SegmentIDs :type "Array of Integer (by ref)")))

(fn `GetGrabber`
  (params (Component :type "SceneComponent Object Reference"))
  (returns (Hand :type "/Game/ESCHER/Blueprints/Elements/VRController Object Reference"))
  (return (`self.Grabber`)))

(fn `IsAutoDropping`
  (params (Component :type "SceneComponent Object Reference"))
  (returns (AutoDrop :type Boolean))
  (return true))

(fn `IsGrabbable`
  (params (Component :type "SceneComponent Object Reference"))
  (returns (Grabbable :type Boolean))
  (return true))

(fn `UserConstructionScript`
  (`parent.UserConstructionScript`))