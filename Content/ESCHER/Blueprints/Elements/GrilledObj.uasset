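; GrilledObj is an actor that dissolves a physics object and then destroys itself.
; On BeginPlay it attaches a DissolveDust emitter to the main mesh and applies a NoBounce physical material.
; After a short delay, a timeline drives the Dissolve material parameter on its meshes and ghost mesh parts.
; Each timeline update also damps linear and angular velocity, slowing the object as it fades.
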(event `self.ReceiveBeginPlay`
  (bind _mainmesh (`self.MainMesh`))
  (bind _mainmesh_2 (`self.MainMesh`))
  (`|ExecutionSequence`
    (:`then_0`
      (`KismetSystemLibrary.Delay` 0.5)
      (bind (_direction _amount) (`Timeline|GrillEffectTimeline`)
        (:`Update`
          (`|ExecutionSequence`
            (:`then_0`
              (for _array_element (`self.Meshes`)
                (`MeshComponent.SetScalarParameterValueOnMaterials` _array_element "Dissolve" _amount))
              (for _array_element_2 (`self.Ghosts`)
                (bind _values (`BlueprintMapLibrary.Map_Values` (`/Game/ESCHER/Blueprints/Elements/GhostObj.NamedParts` _array_element_2)))
                (for _array_element_3 _values
                  (bind _asmesh_component (cast `MeshComponent` _array_element_3))
                  (`MeshComponent.SetScalarParameterValueOnMaterials` _asmesh_component "Dissolve" _amount))))
            (:`then_1`
              (`PrimitiveComponent.SetPhysicsLinearVelocity` _mainmesh_2 (* (`SceneComponent.GetComponentVelocity` _mainmesh_2) 0.95) false "None")
              (`PrimitiveComponent.SetPhysicsAngularVelocityInRadians` _mainmesh (* (`PrimitiveComponent.GetPhysicsAngularVelocityInRadians` _mainmesh "None") 0.95) false "None"))))
        (:`Finished`
          (`self.K2_DestroyActor`))))
    (:`then_1`
      (bind _returnvalue (`|SpawnActorFromClass` "/Game/ESCHER/Blueprints/Elements/GhostableEmitter.GhostableEmitter_C" (`SceneComponent.K2_GetComponentToWorld` (`self.MainMesh`)) "Undefined" "OverrideRootScale" self "/Game/ESCHER/Particles/DissolveDust.DissolveDust" null))
      (`self.K2_AttachToComponent` _returnvalue (`self.MainMesh`) "None" "KeepWorld" "KeepWorld" "KeepWorld" false)
      (`PrimitiveComponent.SetPhysMaterialOverride` (`self.MainMesh`) "/Game/ESCHER/PhysMaterials/NoBounce.NoBounce"))))

(fn `UserConstructionScript`)