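; GhostableEmitter is a one-shot particle effect actor that can be mirrored by a ghost copy in another transform frame.
; Construction applies the chosen emitter template, and the actor destroys itself when the system finishes.
; CreateGhost spawns a far-off ghost object with a matching emitter attached, stored as a named part.
; UpdateGhost re-parents the source transform between the given frames onto that part and copies its active and visibility states.
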(event `self.ReceiveBeginPlay`
  (add `ParticleSystemComponent.OnSystemFinished` (`self.Emitter`) (delegate `Finished`)))

(event `Finished`
  (params (PSystem :type "ParticleSystemComponent Object Reference"))
  (`self.K2_DestroyActor`))

(event `/Game/ESCHER/Blueprints/Core/Ghostable.UpdateGhost`
  (params (Ghost :type "/Game/ESCHER/Blueprints/Elements/GhostObj Object Reference") (From :type "Transform Structure") (To :type "Transform Structure"))
  (bind _emitter (`self.Emitter`))
  (bind _value (`BlueprintMapLibrary.Map_Find` (`/Game/ESCHER/Blueprints/Elements/GhostObj.NamedParts` Ghost) "Emitter"))
  (`SceneComponent.K2_SetWorldTransform` _value (`/Game/ESCHER/Blueprints/Core/BasicMacros.ReParentTransform` (`SceneComponent.K2_GetComponentToWorld` (`self.Emitter`)) From To) false false)
  (`ActorComponent.SetActive` _value (`ActorComponent.IsActive` _emitter) false)
  (`SceneComponent.SetVisibility` _value (`SceneComponent.bVisible` _emitter) false))

(fn `CreateGhost`
  (returns (Ghost :type "/Game/ESCHER/Blueprints/Elements/GhostObj Object Reference"))
  (bind _returnvalue (`|SpawnActorFromClass` "/Game/ESCHER/Blueprints/Elements/GhostObj.GhostObj_C" (`KismetMathLibrary.MakeTransform` (1000000.0 1000000.0 1000000.0)) "Undefined" "OverrideRootScale" null null))
  (bind _returnvalue_2 (`GameplayStatics.SpawnEmitterAttached` (`self.EmitterType`) (`/Game/ESCHER/Blueprints/Elements/GhostObj.Scene` _returnvalue)))
  (`BlueprintMapLibrary.Map_Add` (`/Game/ESCHER/Blueprints/Elements/GhostObj.NamedParts` _returnvalue) "Emitter" _returnvalue_2)
  (return _returnvalue))

(fn `UserConstructionScript`
  (`ParticleSystemComponent.SetTemplate` (`self.Emitter`) (`self.EmitterType`)))