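; One node in a tree of persistent ray segments, tracing a line each update through its Handler and tracking which components it passes or is blocked by.
; It diffs hits against the last known sets to send begin and end events to the Handler and PersistentRayDetecting actors, which can turn a pass into a block.
; Updates recurse into child segments; Destroy recursively tears down children, ends active hits and detaches from the parent or finishes the ray.
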(fn `Destroy`
  (bind _handler (`self.Handler`))
  (bind _handler_2 (`self.Handler`))
  (bind _handler_3 (`self.Handler`))
  (bind _handler_4 (`self.Handler`))
  (bind _parentsegment (`self.ParentSegment`))
  (bind _handler_5 (`self.Handler`))
  (bind _childsegments (`/Game/ESCHER/Blueprints/Elements/PersistentRaySegment.ChildSegments` _parentsegment))
  (if (not (`self.Destroyed`))
    (set `self.Destroyed` true)
    (bind (_arrayindex _arrayelement) (`/Engine/EditorBlueprintResources/StandardMacros.ReverseForEachLoop` (`self.ChildSegmentList`))
      (:`LoopBody`
        (`self.Destroy` _arrayelement))
      (:`Completed`
        (`|ExecutionSequence`
          (:`then_0`
            (`|ExecutionSequence`
              (:`then_0`
                (bind _keys (`BlueprintMapLibrary.Map_Keys` (`self.LastBlockedComponents`)))
                (for _array_element _keys
                  (`/Game/ESCHER/Blueprints/Elements/PersistentRayHandler.OnRayEndedBlock` _handler_2 _handler_2 self _array_element)
                  (bind _aspersistent_ray_detecting (cast `/Game/ESCHER/Blueprints/Core/PersistentRayDetecting` (`ActorComponent.GetOwner` _array_element)))
                  (`/Game/ESCHER/Blueprints/Core/PersistentRayDetecting.EndedBlockPRay` _aspersistent_ray_detecting _array_element self (`self.Handler`))))
              (:`then_1`
                (bind _keys_2 (`BlueprintMapLibrary.Map_Keys` (`self.LastPassedComponents`)))
                (for _array_element_2 _keys_2
                  (`/Game/ESCHER/Blueprints/Elements/PersistentRayHandler.OnRayEndedPass` _handler_3 _handler_3 self _array_element_2)
                  (bind _aspersistent_ray_detecting_2 (cast `/Game/ESCHER/Blueprints/Core/PersistentRayDetecting` (`ActorComponent.GetOwner` _array_element_2)))
                  (`/Game/ESCHER/Blueprints/Core/PersistentRayDetecting.EndedPassPRay` _aspersistent_ray_detecting_2 _array_element_2 self (`self.Handler`))))))
          (:`then_1`
            (if (`self.IsRoot`)
              (set `/Game/ESCHER/Blueprints/Elements/PersistentRayHandler.RootSegment` null _handler_5)
              (set `/Game/ESCHER/Blueprints/Elements/PersistentRayHandler.RayActive` false _handler_5)
              (else
                (`BlueprintMapLibrary.Map_Remove` _childsegments (`self.SegmentID`))
                (bind _values (`BlueprintMapLibrary.Map_Values` _childsegments))
                (set `/Game/ESCHER/Blueprints/Elements/PersistentRaySegment.ChildSegmentList` _values _parentsegment))))
          (:`then_2`
            (`self.OnSegmentDestroyed` self self)
            (`/Game/ESCHER/Blueprints/Elements/PersistentRayHandler.OnSegmentDestroyed` _handler_4 _handler_4 self))
          (:`then_3`
            (if (`self.IsRoot`)
              (`/Game/ESCHER/Blueprints/Elements/PersistentRayHandler.OnRayFinished` _handler _handler))))))))

(fn `Init`
  (bind _parentsegment (`self.ParentSegment`))
  (bind _output_get (set `self.IsRoot` (not (`KismetSystemLibrary.IsValid` (`self.ParentSegment`)))))
  (if (not _output_get)
    (set `self.Depth` (+ (`/Game/ESCHER/Blueprints/Elements/PersistentRaySegment.Depth` _parentsegment) 1))
    (`BlueprintMapLibrary.Map_Add` (`/Game/ESCHER/Blueprints/Elements/PersistentRaySegment.ChildSegments` _parentsegment) (`self.SegmentID`) self)
    (`KismetArrayLibrary.Array_Add` (`/Game/ESCHER/Blueprints/Elements/PersistentRaySegment.ChildSegmentList` _parentsegment) self)))

(fn `UpdatePRaySegment`
  (locals (CurrentHit :type "HitResult Structure") (CurrentHitActor :type "Actor Object Reference") (CurrentHitComponent :type "PrimitiveComponent Object Reference") (ConfirmedBlockedComponents :type "Set of PrimitiveComponent Object Reference") (ConfirmedPassedComponents :type "Set of PrimitiveComponent Object Reference"))
  (bind _currenthit (`local.CurrentHit`))
  (bind _handler (`self.Handler`))
  (bind _currenthit_2 (`local.CurrentHit`))
  (bind _handler_2 (`self.Handler`))
  (bind _sourcelocation (`self.SourceLocation`))
  (bind _handler_3 (`self.Handler`))
  (bind _handler_4 (`self.Handler`))
  (bind _handler_5 (`self.Handler`))
  (bind _handler_6 (`self.Handler`))
  (bind _returnvalue (+ _sourcelocation (* (`self.Towards`) (`self.Distance`))))
  (if (`self.Destroyed`)
    (`KismetSystemLibrary.PrintString` null "Destroyed persistant ray being updated!" true true (struct :`R` 1.0 :`G` 0.089693 :`A` 1.0) 6.0)
    (else
      (`|ExecutionSequence`
        (:`then_0`
          ;[1 1 1] Handle Hitscan Logic
          (set `self.EndLocation` _returnvalue)
          (bind _outhits (`/Game/ESCHER/Blueprints/Elements/PersistentRayHandler.DoLineTrace` (`self.Handler`) _sourcelocation _returnvalue (`self.ActorsToIgnore`)))
          (for _array_element _outhits
            (set `local.CurrentHit` _array_element)
            (bind (_bblockinghit _binitialoverlap _time _distance _location _impactpoint _normal _impactnormal _physmat _hitactor _hitcomponent) (`GameplayStatics.BreakHitResult` _array_element))
            (if (not (`BlueprintSetLibrary.Set_Contains` (`self.ComponentsToIgnore`) _hitcomponent))
              (set `local.CurrentHitActor` _hitactor)
              (set `local.CurrentHitComponent` _hitcomponent)
              (if _bblockinghit
                (`|ExecutionSequence`
                  (:`then_0`
                    (`|ExecutionSequence`
                      (:`then_0`
                        (if (not (`BlueprintMapLibrary.Map_Contains` (`self.LastBlockedComponents`) (`local.CurrentHitComponent`)))
                          (bind _aspersistent_ray_detecting (cast `/Game/ESCHER/Blueprints/Core/PersistentRayDetecting` (`local.CurrentHitActor`))
                            (:`then`
                              (bind (_do_effects _terminal) (`/Game/ESCHER/Blueprints/Core/PersistentRayDetecting.BeganBlockPRay` _aspersistent_ray_detecting (`local.CurrentHit`) self (`self.Handler`)))
                              (`/Game/ESCHER/Blueprints/Elements/PersistentRayHandler.OnRayBeganBlock` _handler_2 _handler_2 self _currenthit _do_effects _terminal))
                            (:`CastFailed`
                              (`/Game/ESCHER/Blueprints/Elements/PersistentRayHandler.OnRayBeganBlock` _handler_2 _handler_2 self _currenthit true true)))))
                      (:`then_1`
                        (`BlueprintMapLibrary.Map_Add` (`self.LastBlockedComponents`) (`local.CurrentHitComponent`) (`local.CurrentHit`))
                        (`BlueprintSetLibrary.Set_Add` (`local.ConfirmedBlockedComponents`) (`local.CurrentHitComponent`)))))
                  (:`then_1`
                    (set `self.EndLocation` _location)
                    (break)))
                (else
                  (`|ExecutionSequence`
                    (:`then_0`
                      (if (`BlueprintMapLibrary.Map_Contains` (`self.LastPassedComponents`) (`local.CurrentHitComponent`))
                        (bind _aspersistent_ray_detecting_2 (cast `/Game/ESCHER/Blueprints/Core/PersistentRayDetecting` (`local.CurrentHitActor`)))
                        (bind _block (`/Game/ESCHER/Blueprints/Core/PersistentRayDetecting.IsPRPassBlocking` _aspersistent_ray_detecting_2 (`local.CurrentHitComponent`) self))
                        (if _block
                          (set `self.EndLocation` _location :!label _label)
                          (break))
                        (else
                          (bind _aspersistent_ray_detecting_3 (cast `/Game/ESCHER/Blueprints/Core/PersistentRayDetecting` _hitactor)
                            (:`then`
                              (bind (_doeffects _shouldblock _terminal_2) (`/Game/ESCHER/Blueprints/Core/PersistentRayDetecting.BeganPassPRay` _aspersistent_ray_detecting_3 (`local.CurrentHit`) self (`self.Handler`)))
                              (if _shouldblock
                                (`/Game/ESCHER/Blueprints/Elements/PersistentRayHandler.OnRayBeganBlock` _handler (`self.Handler`) self (`local.CurrentHit`) _doeffects _terminal_2)
                                (goto _label)
                                (else
                                  (`/Game/ESCHER/Blueprints/Elements/PersistentRayHandler.OnRayBeganPass` _handler _handler self _currenthit_2 _doeffects))))
                            (:`CastFailed`
                              (`/Game/ESCHER/Blueprints/Elements/PersistentRayHandler.OnRayBeganPass` _handler _handler self _currenthit_2 true))))))
                    (:`then_1`
                      (`BlueprintMapLibrary.Map_Add` (`self.LastPassedComponents`) (`local.CurrentHitComponent`) (`local.CurrentHit`)) ; Update hit value
                      (`BlueprintSetLibrary.Set_Add` (`local.ConfirmedPassedComponents`) (`local.CurrentHitComponent`)))))))))
        (:`then_1`
          ;[1 1 1] Handle Ended Hits
          (`|ExecutionSequence`
            (:`then_0`
              (bind _keys (`BlueprintMapLibrary.Map_Keys` (`self.LastBlockedComponents`)))
              (bind (_arrayindex _arrayelement) (`/Engine/EditorBlueprintResources/StandardMacros.ReverseForEachLoop` _keys)
                (:`LoopBody`
                  (if (not (`BlueprintSetLibrary.Set_Contains` (`local.ConfirmedBlockedComponents`) _arrayelement))
                    (`BlueprintMapLibrary.Map_Remove` (`self.LastBlockedComponents`) _arrayelement)
                    (`/Game/ESCHER/Blueprints/Elements/PersistentRayHandler.OnRayEndedBlock` _handler_4 _handler_4 self _arrayelement)
                    (bind _aspersistent_ray_detecting_4 (cast `/Game/ESCHER/Blueprints/Core/PersistentRayDetecting` (`ActorComponent.GetOwner` _arrayelement)))
                    (`/Game/ESCHER/Blueprints/Core/PersistentRayDetecting.EndedBlockPRay` _aspersistent_ray_detecting_4 _arrayelement self (`self.Handler`))))))
            (:`then_1`
              (bind _keys_2 (`BlueprintMapLibrary.Map_Keys` (`self.LastPassedComponents`)))
              (bind (_arrayindex_2 _arrayelement_2) (`/Engine/EditorBlueprintResources/StandardMacros.ReverseForEachLoop` _keys_2)
                (:`LoopBody`
                  (if (not (`BlueprintSetLibrary.Set_Contains` (`local.ConfirmedPassedComponents`) _arrayelement_2))
                    (`BlueprintMapLibrary.Map_Remove` (`self.LastPassedComponents`) _arrayelement_2)
                    (`/Game/ESCHER/Blueprints/Elements/PersistentRayHandler.OnRayEndedPass` _handler_3 _handler_3 self _arrayelement_2)
                    (bind _aspersistent_ray_detecting_5 (cast `/Game/ESCHER/Blueprints/Core/PersistentRayDetecting` (`ActorComponent.GetOwner` _arrayelement_2)))
                    (`/Game/ESCHER/Blueprints/Core/PersistentRayDetecting.EndedPassPRay` _aspersistent_ray_detecting_5 _arrayelement_2 self (`self.Handler`))))))))
        (:`then_2`
          ;[1 1 1] Update Children
          (`self.UpdatePostSelfPreChildren` self)
          (`/Game/ESCHER/Blueprints/Elements/PersistentRayHandler.OnSegmentUpdatePostSelfPreChildren` _handler_6 _handler_6 self)
          (for _array_element_2 (`self.ChildSegmentList`)
            (`self.UpdatePRaySegment` _array_element_2)))
        (:`then_3`
          (set `/Game/ESCHER/Blueprints/Elements/PersistentRayHandler.LastRootSourceLocation` (`self.SourceLocation`) _handler_5)
          (set `/Game/ESCHER/Blueprints/Elements/PersistentRayHandler.LastRootTowards` (`self.Towards`) _handler_5))))))