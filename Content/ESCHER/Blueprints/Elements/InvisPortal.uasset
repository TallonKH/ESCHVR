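; InvisPortal is a two-sided portal that carries Portalable actors and rays between PortA and PortB.
; Tick teleports tracked overlapping actors once their origin crosses a portal plane, and PreTeleportThrough re-parents the VR pawn's check vectors.
; One-shot rays fire a re-parented segment from the opposite side with remaining distance.
; Persistent rays keep a mapped child segment per side, updated through bound segment events and removed when the ray leaves.
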(event `self.FarA.OnComponentBeginOverlap`
  (params (OverlappedComponent :type "PrimitiveComponent Object Reference") (OtherActor :type "Actor Object Reference") (OtherComp :type "PrimitiveComponent Object Reference") (OtherBodyIndex :type Integer) (bFromSweep :type Boolean) (SweepResult :type "HitResult Structure (by ref)"))
  ;[1 1 1] Handle Portalables
  (cast `/Game/ESCHER/Blueprints/Core/Portalable` OtherActor)
  (`BlueprintSetLibrary.Set_Add` (`self.TrackedAPortalables`) OtherActor))

(event `self.FarA.OnComponentEndOverlap`
  (params (OverlappedComponent :type "PrimitiveComponent Object Reference") (OtherActor :type "Actor Object Reference") (OtherComp :type "PrimitiveComponent Object Reference") (OtherBodyIndex :type Integer))
  ;[1 1 1] Handle Portalables
  (`BlueprintSetLibrary.Set_Remove` (`self.TrackedAPortalables`) OtherActor))

(event `self.FarB.OnComponentBeginOverlap`
  (params (OverlappedComponent :type "PrimitiveComponent Object Reference") (OtherActor :type "Actor Object Reference") (OtherComp :type "PrimitiveComponent Object Reference") (OtherBodyIndex :type Integer) (bFromSweep :type Boolean) (SweepResult :type "HitResult Structure (by ref)"))
  ;[1 1 1] Handle Portalables
  (cast `/Game/ESCHER/Blueprints/Core/Portalable` OtherActor)
  (`BlueprintSetLibrary.Set_Add` (`self.TrackedBPortalables`) OtherActor))

(event `self.FarB.OnComponentEndOverlap`
  (params (OverlappedComponent :type "PrimitiveComponent Object Reference") (OtherActor :type "Actor Object Reference") (OtherComp :type "PrimitiveComponent Object Reference") (OtherBodyIndex :type Integer))
  ;[1 1 1] Handle Portalables
  (`BlueprintSetLibrary.Set_Remove` (`self.TrackedBPortalables`) OtherActor))

(event `/Game/ESCHER/Blueprints/Core/TeleportListener.PreTeleportThrough`
  (params (VRPawn :type "/Game/ESCHER/Blueprints/Elements/VRPawn Object Reference") (Hit :type "HitResult Structure"))
  (bind _porta (`self.PortA`))
  (bind _portb (`self.PortB`))
  (bind _returnvalue (== (`.HitComponent` (`GameplayStatics.BreakHitResult` Hit)) (`self.PortA`)))
  (bind _returnvalue_2 (`SceneComponent.K2_GetComponentToWorld` (select `bool` _returnvalue :`false` _portb :`true` _porta :!type "PrimitiveComponent Object Reference")))
  (bind _returnvalue_3 (`SceneComponent.K2_GetComponentToWorld` (select `bool` _returnvalue :`false` _porta :`true` _portb :!type "PrimitiveComponent Object Reference")))
  (set `/Game/ESCHER/Blueprints/Elements/VRPawn.CTPResetProxies` true VRPawn)
  (set `/Game/ESCHER/Blueprints/Elements/VRPawn.CTPCheckNormal` (`/Game/ESCHER/Blueprints/Core/BasicMacros.ReParentVector` (`/Game/ESCHER/Blueprints/Elements/VRPawn.CTPCheckNormal` VRPawn) _returnvalue_2 _returnvalue_3) VRPawn)
  (set `/Game/ESCHER/Blueprints/Elements/VRPawn.CTPForwardVector` (`/Game/ESCHER/Blueprints/Core/BasicMacros.ReParentVector` (`/Game/ESCHER/Blueprints/Elements/VRPawn.CTPForwardVector` VRPawn) _returnvalue_2 _returnvalue_3) VRPawn))

(event `self.ReceiveTick`
  (params (DeltaSeconds :type "Float (single-precision)"))
  (bind _porta (`self.PortA`))
  (bind _portb (`self.PortB`))
  ;[1 1 1] Handle Portalables
  (`|ExecutionSequence`
    (:`then_0`
      (bind _result (`BlueprintSetLibrary.Set_ToArray` (`self.TrackedAPortalables`)))
      (for _array_element _result
        (bind _asportalable (cast `/Game/ESCHER/Blueprints/Core/Portalable` _array_element))
        (bind _origin (`/Game/ESCHER/Blueprints/Core/Portalable.Get Origin` _asportalable))
        (if (< (`KismetMathLibrary.Dot_VectorVector` (- _origin (`SceneComponent.K2_GetComponentLocation` _porta)) (`SceneComponent.GetForwardVector` _porta)) 0.0)
          (`/Game/ESCHER/Blueprints/Core/Portalable.Teleport` _asportalable self false (`SceneComponent.K2_GetComponentToWorld` (`self.PortA`)) (`SceneComponent.K2_GetComponentToWorld` (`self.PortB`))))))
    (:`then_1`
      (bind _result_2 (`BlueprintSetLibrary.Set_ToArray` (`self.TrackedBPortalables`)))
      (for _array_element_2 _result_2
        (bind _asportalable_2 (cast `/Game/ESCHER/Blueprints/Core/Portalable` _array_element_2))
        (bind _origin_2 (`/Game/ESCHER/Blueprints/Core/Portalable.Get Origin` _asportalable_2))
        (if (> (`KismetMathLibrary.Dot_VectorVector` (- _origin_2 (`SceneComponent.K2_GetComponentLocation` _portb)) (`SceneComponent.GetForwardVector` _portb)) 0.0)
          (`/Game/ESCHER/Blueprints/Core/Portalable.Teleport` _asportalable_2 self true (`SceneComponent.K2_GetComponentToWorld` (`self.PortB`)) (`SceneComponent.K2_GetComponentToWorld` (`self.PortA`))))))))

(event `self.EndedPassPRay`
  (params (UnhitComponent :type "PrimitiveComponent Object Reference") (Segment :type "/Game/ESCHER/Blueprints/Elements/PersistentRaySegment Object Reference") (Handler :type "/Game/ESCHER/Blueprints/Elements/PersistentRayHandler Object Reference"))
  (bind _value (`BlueprintMapLibrary.Map_Find` (`self.TrackedBPSegments`) Segment))
  (bind _value_2 (`BlueprintMapLibrary.Map_Find` (`self.TrackedAPSegments`) Segment))
  ;[1 1 1] Handle Persistent Ray Events
  (if (== UnhitComponent (`self.PortA`))
    (`/Engine/EditorBlueprintResources/StandardMacros.IsValid` _value_2
      (:`Is Valid`
        (set `self.ToDelete` _value_2)
        (`BlueprintMapLibrary.Map_Remove` (`self.TrackedAPSegments`) Segment)
        (remove `/Game/ESCHER/Blueprints/Elements/PersistentRaySegment.UpdatePostSelfPreChildren` Segment (delegate `TracedPASegUpdated`))
        (remove `/Game/ESCHER/Blueprints/Elements/PersistentRaySegment.OnSegmentDestroyed` Segment (delegate `TracedPASegmentDestroyed`))
        (`/Game/ESCHER/Blueprints/Elements/PersistentRaySegment.Destroy` (`self.ToDelete`))))
    (else
      (`/Engine/EditorBlueprintResources/StandardMacros.IsValid` _value
        (:`Is Valid`
          (set `self.ToDelete` _value)
          (`BlueprintMapLibrary.Map_Remove` (`self.TrackedBPSegments`) Segment)
          (remove `/Game/ESCHER/Blueprints/Elements/PersistentRaySegment.UpdatePostSelfPreChildren` Segment (delegate `TracedPBSegmentUpdated`))
          (remove `/Game/ESCHER/Blueprints/Elements/PersistentRaySegment.OnSegmentDestroyed` Segment (delegate `TracedPBSegmentDestroyed`))
          (`/Game/ESCHER/Blueprints/Elements/PersistentRaySegment.Destroy` (`self.ToDelete`)))))))

(event `BindPASegmentEvents`
  (params (Parent :type "/Game/ESCHER/Blueprints/Elements/PersistentRaySegment Object Reference"))
  ;[1 1 1] Handle Persistent Ray Events
  (add `/Game/ESCHER/Blueprints/Elements/PersistentRaySegment.UpdatePostSelfPreChildren` Parent (delegate `TracedPASegUpdated`))
  (add `/Game/ESCHER/Blueprints/Elements/PersistentRaySegment.OnSegmentDestroyed` Parent (delegate `TracedPASegmentDestroyed`)))

(event `TracedPASegmentDestroyed`
  (params (Segment :type "/Game/ESCHER/Blueprints/Elements/PersistentRaySegment Object Reference"))
  ;[1 1 1] Handle Persistent Ray Events
  (`BlueprintMapLibrary.Map_Remove` (`self.TrackedAPSegments`) Segment)
  (remove `/Game/ESCHER/Blueprints/Elements/PersistentRaySegment.UpdatePostSelfPreChildren` Segment (delegate `TracedPASegUpdated`))
  (remove `/Game/ESCHER/Blueprints/Elements/PersistentRaySegment.OnSegmentDestroyed` Segment (delegate `TracedPASegmentDestroyed`)))

(event `TracedPASegUpdated`
  (params (UpdatedSegment :type "/Game/ESCHER/Blueprints/Elements/PersistentRaySegment Object Reference"))
  (bind _trackedapsegments (`self.TrackedAPSegments`))
  (bind _currentpseg (`self.CurrentPSeg`))
  (bind _currentpseg_2 (`self.CurrentPSeg`))
  (bind _value (`BlueprintMapLibrary.Map_Find` (`self.TrackedAPSegments`) _currentpseg_2))
  (bind (_bblockinghit _binitialoverlap _time _distance _location) (`GameplayStatics.BreakHitResult` (`self.CurrentSegHit`)))
  (bind _value_2 (`BlueprintMapLibrary.Map_Find` _trackedapsegments (`self.CurrentPSeg`)))
  (bind _returnvalue (`SceneComponent.K2_GetComponentToWorld` (`self.CurrentSegEntrySide`)))
  (bind _returnvalue_2 (`SceneComponent.K2_GetComponentToWorld` (`self.CurrentSegExitSide`)))
  (bind _returnvalue_3 (+ (`/Game/ESCHER/Blueprints/Elements/PersistentRaySegment.AccumulatedDistance` _currentpseg_2) _distance))
  ;[1 1 1] Handle Persistent Ray Events
  ;;[1 1 1] A Side Ray Updates
  (set `self.CurrentPSeg` UpdatedSegment)
  (set `self.CurrentSegHit` (`BlueprintMapLibrary.Map_Find` (`/Game/ESCHER/Blueprints/Elements/PersistentRaySegment.LastPassedComponents` (`self.CurrentPSeg`)) (`self.PortA`)))
  (set `self.CurrentSide` true)
  (set `self.CurrentSegEntrySide` (`self.PortA`))
  (set `self.CurrentSegExitSide` (`self.PortB`))
  (set `self.CurrentSegChild` (`BlueprintMapLibrary.Map_Find` (`self.TrackedAPSegments`) (`self.CurrentPSeg`)))
  (if (< (`KismetMathLibrary.Dot_VectorVector` (`/Game/ESCHER/Blueprints/Elements/PersistentRaySegment.Towards` (`self.CurrentPSeg`)) (`SceneComponent.GetForwardVector` (`self.CurrentSegEntrySide`))) 0.0)
    (`|ExecutionSequence`
      (:`then_0`
        (if (not (`BlueprintMapLibrary.Map_Contains` (`self.TrackedAPSegments`) (`self.CurrentPSeg`)))
          (bind _segment (`/Game/ESCHER/Blueprints/Elements/PersistentRayHandler.CreateSegment` (`/Game/ESCHER/Blueprints/Elements/PersistentRaySegment.Handler` _currentpseg) _currentpseg))
          (`BlueprintMapLibrary.Map_Add` (`self.TrackedAPSegments`) _currentpseg _segment)
          (`BlueprintSetLibrary.Set_Add` (`/Game/ESCHER/Blueprints/Elements/PersistentRaySegment.ComponentsToIgnore` _segment) (`self.PortB`))))
      (:`then_1`
        (set `/Game/ESCHER/Blueprints/Elements/PersistentRaySegment.SourceLocation` (`/Game/ESCHER/Blueprints/Core/BasicMacros.ReParentPosition` _location _returnvalue _returnvalue_2) _value)
        (set `/Game/ESCHER/Blueprints/Elements/PersistentRaySegment.Towards` (`/Game/ESCHER/Blueprints/Core/BasicMacros.ReParentVector` (`/Game/ESCHER/Blueprints/Elements/PersistentRaySegment.Towards` (`self.CurrentPSeg`)) _returnvalue _returnvalue_2) _value)
        (set `/Game/ESCHER/Blueprints/Elements/PersistentRaySegment.Distance` (- (`/Game/ESCHER/Blueprints/Elements/PersistentRayHandler.MaxDistance` (`/Game/ESCHER/Blueprints/Elements/PersistentRaySegment.Handler` _currentpseg_2)) _returnvalue_3) _value)
        (set `/Game/ESCHER/Blueprints/Elements/PersistentRaySegment.AccumulatedDistance` _returnvalue_3 _value)))
    (else
      (`/Engine/EditorBlueprintResources/StandardMacros.IsValid` _value_2
        (:`Is Valid`
          (`/Game/ESCHER/Blueprints/Elements/PersistentRaySegment.Destroy` _value_2)
          (`BlueprintMapLibrary.Map_Remove` _trackedapsegments _value_2))))))

(event `BindPBSegmentEvents`
  (params (Parent :type "/Game/ESCHER/Blueprints/Elements/PersistentRaySegment Object Reference"))
  ;[1 1 1] Handle Persistent Ray Events
  (add `/Game/ESCHER/Blueprints/Elements/PersistentRaySegment.UpdatePostSelfPreChildren` Parent (delegate `TracedPBSegmentUpdated`))
  (add `/Game/ESCHER/Blueprints/Elements/PersistentRaySegment.OnSegmentDestroyed` Parent (delegate `TracedPBSegmentDestroyed`)))

(event `TracedPBSegmentDestroyed`
  (params (Segment :type "/Game/ESCHER/Blueprints/Elements/PersistentRaySegment Object Reference"))
  ;[1 1 1] Handle Persistent Ray Events
  (`BlueprintMapLibrary.Map_Remove` (`self.TrackedBPSegments`) Segment)
  (remove `/Game/ESCHER/Blueprints/Elements/PersistentRaySegment.UpdatePostSelfPreChildren` Segment (delegate `TracedPBSegmentUpdated`))
  (remove `/Game/ESCHER/Blueprints/Elements/PersistentRaySegment.OnSegmentDestroyed` Segment (delegate `TracedPBSegmentDestroyed`)))

(event `TracedPBSegmentUpdated`
  (params (UpdatedSegment :type "/Game/ESCHER/Blueprints/Elements/PersistentRaySegment Object Reference"))
  (bind _currentpseg (`self.CurrentPSeg`))
  (bind _currentpseg_2 (`self.CurrentPSeg`))
  (bind _trackedbpsegments (`self.TrackedBPSegments`))
  (bind (_bblockinghit _binitialoverlap _time _distance _location) (`GameplayStatics.BreakHitResult` (`self.CurrentSegHit`)))
  (bind _returnvalue (`SceneComponent.K2_GetComponentToWorld` (`self.CurrentSegEntrySide`)))
  (bind _returnvalue_2 (`SceneComponent.K2_GetComponentToWorld` (`self.CurrentSegExitSide`)))
  (bind _value (`BlueprintMapLibrary.Map_Find` _trackedbpsegments (`self.CurrentPSeg`)))
  (bind _value_2 (`BlueprintMapLibrary.Map_Find` (`self.TrackedBPSegments`) _currentpseg_2))
  (bind _returnvalue_3 (+ (`/Game/ESCHER/Blueprints/Elements/PersistentRaySegment.AccumulatedDistance` _currentpseg_2) _distance))
  ;[1 1 1] Handle Persistent Ray Events
  ;;[1 1 1] B Side Ray Updates
  (set `self.CurrentPSeg` UpdatedSegment)
  (set `self.CurrentSegHit` (`BlueprintMapLibrary.Map_Find` (`/Game/ESCHER/Blueprints/Elements/PersistentRaySegment.LastPassedComponents` (`self.CurrentPSeg`)) (`self.PortB`)))
  (set `self.CurrentSide` false)
  (set `self.CurrentSegEntrySide` (`self.PortB`))
  (set `self.CurrentSegExitSide` (`self.PortA`))
  (set `self.CurrentSegChild` (`BlueprintMapLibrary.Map_Find` (`self.TrackedBPSegments`) (`self.CurrentPSeg`)))
  (if (> (`KismetMathLibrary.Dot_VectorVector` (`/Game/ESCHER/Blueprints/Elements/PersistentRaySegment.Towards` (`self.CurrentPSeg`)) (`SceneComponent.GetForwardVector` (`self.CurrentSegEntrySide`))) 0.0)
    (`|ExecutionSequence`
      (:`then_0`
        (if (not (`BlueprintMapLibrary.Map_Contains` (`self.TrackedBPSegments`) (`self.CurrentPSeg`)))
          (bind _segment (`/Game/ESCHER/Blueprints/Elements/PersistentRayHandler.CreateSegment` (`/Game/ESCHER/Blueprints/Elements/PersistentRaySegment.Handler` _currentpseg) _currentpseg))
          (`BlueprintMapLibrary.Map_Add` (`self.TrackedBPSegments`) _currentpseg _segment)
          (`BlueprintSetLibrary.Set_Add` (`/Game/ESCHER/Blueprints/Elements/PersistentRaySegment.ComponentsToIgnore` _segment) (`self.PortA`))))
      (:`then_1`
        (set `/Game/ESCHER/Blueprints/Elements/PersistentRaySegment.SourceLocation` (`/Game/ESCHER/Blueprints/Core/BasicMacros.ReParentPosition` _location _returnvalue _returnvalue_2) _value_2)
        (set `/Game/ESCHER/Blueprints/Elements/PersistentRaySegment.Towards` (`/Game/ESCHER/Blueprints/Core/BasicMacros.ReParentVector` (`/Game/ESCHER/Blueprints/Elements/PersistentRaySegment.Towards` (`self.CurrentPSeg`)) _returnvalue _returnvalue_2) _value_2)
        (set `/Game/ESCHER/Blueprints/Elements/PersistentRaySegment.Distance` (- (`/Game/ESCHER/Blueprints/Elements/PersistentRayHandler.MaxDistance` (`/Game/ESCHER/Blueprints/Elements/PersistentRaySegment.Handler` _currentpseg_2)) _returnvalue_3) _value_2)
        (set `/Game/ESCHER/Blueprints/Elements/PersistentRaySegment.AccumulatedDistance` _returnvalue_3 _value_2)))
    (else
      (`/Engine/EditorBlueprintResources/StandardMacros.IsValid` _value
        (:`Is Valid`
          (`/Game/ESCHER/Blueprints/Elements/PersistentRaySegment.Destroy` _value)
          (`BlueprintMapLibrary.Map_Remove` _trackedbpsegments _value))))))

(fn `BeganBlockPRay`
  (params (Hit :type "HitResult Structure") (Segment :type "/Game/ESCHER/Blueprints/Elements/PersistentRaySegment Object Reference") (RayHandler :type "/Game/ESCHER/Blueprints/Elements/PersistentRayHandler Object Reference"))
  (returns (`Do Effects` :type Boolean) (Terminal :type Boolean)))

(fn `BeganPassPRay`
  (params (Hit :type "HitResult Structure") (Segment :type "/Game/ESCHER/Blueprints/Elements/PersistentRaySegment Object Reference") (RayHandler :type "/Game/ESCHER/Blueprints/Elements/PersistentRayHandler Object Reference"))
  (returns (DoEffects :type Boolean) (ShouldBlock :type Boolean) (Terminal :type Boolean))
  (bind (_bblockinghit _binitialoverlap _time _distance _location _impactpoint _normal _impactnormal _physmat _hitactor _hitcomponent) (`GameplayStatics.BreakHitResult` Hit))
  (bind _block (`self.IsPRPassBlocking` self _hitcomponent Segment))
  (if _block
    (if (== _hitcomponent (`self.PortA`))
      (`self.BindPASegmentEvents` Segment)
      (else
        (`self.BindPBSegmentEvents` Segment)))
    (return false (`self.IsBlocking`) false)
    (else
      (return false false false))))

(fn `BlockedBRay`
  (params (RayHandler :type "/Game/ESCHER/Blueprints/Elements/BurstRayHandler Object Reference") (SegmentInfo :type "/Game/ESCHER/Blueprints/Core/BurstRaySegmentInfo Structure") (Hit :type "HitResult Structure"))
  (returns (DoEffects :type Boolean) (Terminal :type Boolean))
  (return false false))

(fn `IsPRPassBlocking`
  (params (Component :type "PrimitiveComponent Object Reference") (Segment :type "/Game/ESCHER/Blueprints/Elements/PersistentRaySegment Object Reference"))
  (returns (Block :type Boolean))
  (bind _returnvalue (`KismetMathLibrary.Dot_VectorVector` (`SceneComponent.GetForwardVector` Component) (`/Game/ESCHER/Blueprints/Elements/PersistentRaySegment.Towards` Segment)))
  (return (and (`self.IsBlocking`) (not (and (== (`.Distance` (`GameplayStatics.BreakHitResult` (`BlueprintMapLibrary.Map_Find` (`/Game/ESCHER/Blueprints/Elements/PersistentRaySegment.LastPassedComponents` Segment) Component))) 0.0) (`/Game/ESCHER/Blueprints/Core/BasicMacros.SelectBoolean` (> _returnvalue 0.0) (< _returnvalue 0.0) (== Component (`self.PortA`))))))))

(fn `PassedBRay`
  (params (RayHandler :type "/Game/ESCHER/Blueprints/Elements/BurstRayHandler Object Reference") (SegmentInfo :type "/Game/ESCHER/Blueprints/Core/BurstRaySegmentInfo Structure") (Hit :type "HitResult Structure"))
  (returns (DoEffects :type Boolean) (Block :type Boolean) (Terminal :type Boolean))
  (bind (_depth _accumulateddistance _direction) (break `/Game/ESCHER/Blueprints/Core/BurstRaySegmentInfo` SegmentInfo))
  (bind (_bblockinghit _binitialoverlap _time _distance _location _impactpoint _normal _impactnormal _physmat _hitactor _hitcomponent) (`GameplayStatics.BreakHitResult` Hit))
  (bind _porta (`self.PortA`))
  (bind _portb (`self.PortB`))
  (bind _isblocking (`self.IsBlocking`))
  (bind _returnvalue (== _hitcomponent (`self.PortA`)))
  (bind _returnvalue_2 (+ _accumulateddistance _distance))
  (bind _returnvalue_3 (select `bool` _returnvalue :`false` _portb :`true` _porta :!type "PrimitiveComponent Object Reference"))
  (bind _returnvalue_4 (select `bool` _returnvalue :`false` _porta :`true` _portb :!type "PrimitiveComponent Object Reference"))
  (bind _returnvalue_5 (`SceneComponent.K2_GetComponentToWorld` _returnvalue_3))
  (bind _returnvalue_6 (`SceneComponent.K2_GetComponentToWorld` _returnvalue_4))
  (bind _returnvalue_7 (`KismetMathLibrary.Dot_VectorVector` (`SceneComponent.GetForwardVector` _returnvalue_3) _direction))
  (bind _returnvalue_8 (> _returnvalue_7 0.0))
  (bind _returnvalue_9 (< _returnvalue_7 0.0))
  (if (and (`self.IsBlocking`) (not (and (== _distance 0.0) (`/Game/ESCHER/Blueprints/Core/BasicMacros.SelectBoolean` _returnvalue_8 _returnvalue_9 _returnvalue))))
    (if (`/Game/ESCHER/Blueprints/Core/BasicMacros.SelectBoolean` _returnvalue_9 _returnvalue_8 _returnvalue)
      (`/Game/ESCHER/Blueprints/Elements/BurstRayHandler.SegmentFire` RayHandler (`/Game/ESCHER/Blueprints/Core/BasicMacros.ReParentPosition` _location _returnvalue_5 _returnvalue_6) (`/Game/ESCHER/Blueprints/Core/BasicMacros.ReParentVector` _direction _returnvalue_5 _returnvalue_6) (- (`/Game/ESCHER/Blueprints/Elements/BurstRayHandler.MaxDistance` RayHandler) _returnvalue_2) (+ _depth 1) _returnvalue_2 (`|MakeSet` _returnvalue_4))
      (return false (`self.IsBlocking`) false)
      (else
        (return false _isblocking _isblocking)))
    (else
      (return false false false))))

(fn `UserConstructionScript`)