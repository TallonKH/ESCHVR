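; PhysObj is a physics-driven mesh actor with its own gravity direction that can teleport between two reference frames.
; Each tick it adds LocalDown gravity to its velocity, capped at terminal velocity, after launching with a local-space initial velocity.
; Teleport re-parents transform and linear and angular velocities, while a spawned GhostObj mirrors the mesh in the other frame.
; Slice hides the mesh and cuts a procedural copy into capped halves.
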(event `/Game/ESCHER/Blueprints/Core/Portalable.Teleport`
  (params (Portal :type "/Game/ESCHER/Blueprints/Elements/LevelStructure/InvisPortal Object Reference") (side :type Boolean) (From :type "Transform Structure") (To :type "Transform Structure"))
  (bind _mainmesh (`self.MainMesh`))
  (bind _mainmesh_2 (`self.MainMesh`))
  (`SceneComponent.K2_SetWorldTransform` _mainmesh (`/Game/ESCHER/Blueprints/Core/BasicMacros.ReParentTransform` (`SceneComponent.K2_GetComponentToWorld` _mainmesh) From To) false false)
  (bind _returnvalue (`PrimitiveComponent.GetPhysicsLinearVelocity` _mainmesh_2 "None"))
  (`PrimitiveComponent.SetPhysicsLinearVelocity` _mainmesh_2 (`/Game/ESCHER/Blueprints/Core/BasicMacros.ReParentVector` _returnvalue From To) false "None")
  (`PrimitiveComponent.SetPhysicsAngularVelocityInDegrees` (`self.MainMesh`) (`/Game/ESCHER/Blueprints/Core/BasicMacros.ReParentVector` (`PrimitiveComponent.GetPhysicsAngularVelocityInDegrees` _mainmesh_2 "None") From To) false "None"))

(event `/Game/ESCHER/Blueprints/Core/Ghostable.UpdateGhost`
  (params (Ghost :type "/Game/ESCHER/Blueprints/Elements/GhostObj Object Reference") (From :type "Transform Structure") (To :type "Transform Structure"))
  (`SceneComponent.K2_SetWorldTransform` (`/Game/ESCHER/Blueprints/Elements/GhostObj.GhostMesh` Ghost) (`/Game/ESCHER/Blueprints/Core/BasicMacros.ReParentTransform` (`SceneComponent.K2_GetComponentToWorld` (`self.MainMesh`)) From To) false false))

(event `self.ReceiveTick`
  (params (DeltaSeconds :type "Float (single-precision)"))
  (`parent.ReceiveTick` DeltaSeconds)
  (`self.PhysicsTick`))

(event `self.ReceiveBeginPlay`
  (`PrimitiveComponent.SetPhysicsLinearVelocity` (`self.MainMesh`) (`KismetMathLibrary.TransformDirection` (`SceneComponent.K2_GetComponentToWorld` (`self.MainMesh`)) (`self.InitialVelocity`)) false "None"))

(fn `CreateGhost`
  (returns (Ghost :type "/Game/ESCHER/Blueprints/Elements/GhostObj Object Reference"))
  (bind _returnvalue (`|SpawnActorFromClass` "/Game/ESCHER/Blueprints/Elements/GhostObj.GhostObj_C" (`KismetMathLibrary.MakeTransform` (1000000.0 1000000.0 1000000.0)) "AlwaysSpawn" "OverrideRootScale" null null))
  (`/Game/ESCHER/Blueprints/Core/BasicMacros.CopyMesh` (`self.MainMesh`) (`/Game/ESCHER/Blueprints/Elements/GhostObj.GhostMesh` _returnvalue))
  (return _returnvalue))

(fn `Get Origin`
  (returns (Origin :type "Vector Structure"))
  (return (`SceneComponent.K2_GetComponentLocation` (`self.MainMesh`))))

(fn `PhysicsTick`
  (bind _mainmesh (`self.MainMesh`))
  (`PrimitiveComponent.SetPhysicsLinearVelocity` _mainmesh (`KismetMathLibrary.ClampVectorSize` (+ (`SceneComponent.GetComponentVelocity` _mainmesh) (* (`self.LocalDown`) (* (`self.GravityImpact`) (`GameplayStatics.GetWorldDeltaSeconds`)))) 0.0 (`self.TerminalVelocity`)) false "None"))

(fn `Slice`
  (params (PlanePosition :type "Vector Structure") (PlaneNormal :type "Vector Structure"))
  (bind _mainmesh (`self.MainMesh`))
  (bind _returnvalue (`AddComponent|NODE_AddProceduralMeshComponent-0` :`bManualAttachment` true :`RelativeTransform` (`SceneComponent.GetRelativeTransform` (`self.MainMesh`))))
  (`SceneComponent.K2_AttachToComponent` _returnvalue _mainmesh "None" "KeepWorld" "KeepWorld" "KeepWorld" false)
  (`SceneComponent.SetVisibility` _mainmesh false false)
  (`KismetProceduralMeshLibrary.CopyProceduralMeshFromStaticMeshComponent` _mainmesh 0 _returnvalue true)
  (`KismetProceduralMeshLibrary.SliceProceduralMesh` _returnvalue PlanePosition PlaneNormal true "UseLastSectionForCap" "/Game/ESCHER/Materials/World/FractalGrid.FractalGrid"))

(fn `UserConstructionScript`)