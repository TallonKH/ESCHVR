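; LookDetector is a placeable actor that detects when the VR player's head camera looks at it and broadcasts look started and ended events.
; Every few ticks while active, it checks player distance, angle to its forward axis (either side) and line of sight.
; It intersects the gaze with a camera-facing plane through itself, using a distance-scaled tolerance.
; An optional LookPoint component visualises the gaze point.
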(event `self.ReceiveBeginPlay`
  (bind _asvrpawn (cast `/Game/ESCHER/Blueprints/Elements/Player/VRPawn` (`GameplayStatics.GetPlayerPawn` 0)))
  (set `self.VRPawn` _asvrpawn))

(event `self.ReceiveTick`
  (params (DeltaSeconds :type "Float (single-precision)"))
  (bind _returnvalue (`self.K2_GetActorLocation`))
  (bind _lookedat (`self.LookedAt`))
  (bind _camera (`/Game/ESCHER/Blueprints/Elements/Player/VRHead.Camera` (`/Game/ESCHER/Blueprints/Elements/Player/VRPawn.HeadActor` (`self.VRPawn`))))
  (bind _returnvalue_2 (`SceneComponent.K2_GetComponentLocation` _camera))
  (bind _returnvalue_3 (- _returnvalue_2 _returnvalue))
  (bind _returnvalue_4 (`KismetMathLibrary.VSize` (- _returnvalue_2 _returnvalue)))
  (bind (_t _intersection _returnvalue_5) (`KismetMathLibrary.LinePlaneIntersection_OriginNormal` _returnvalue_2 (+ (* (`SceneComponent.GetForwardVector` _camera) 65536.0) _returnvalue_2) _returnvalue _returnvalue_3))
  (bind _returnvalue_6 (* _returnvalue_4 (`self.LookPrecisionFactor`)))
  (bind _returnvalue_7 (`KismetMathLibrary.VSizeSquared` (- _returnvalue _intersection)))
  (if (`self.Active`)
    (bind _result (`/Engine/EditorBlueprintResources/StandardMacros.IncrementInt` (`self.TickCounter`))
      (:`  `
        (if (>= _result (`self.TickFrequency`))
          (set `self.TickCounter` 0)
          (`|ExecutionSequence`
            (:`then_0`
              (if (`self.DrawLookPoint`)
                (`SceneComponent.K2_SetWorldLocation` (`self.LookPoint`) _intersection false false)))
            (:`then_1`
              (if (<= _returnvalue_4 (`self.MaxPlayerDistance`))
                (if (<= (`KismetMathLibrary.DegAcos` (`KismetMathLibrary.Abs` (`KismetMathLibrary.Dot_VectorVector` (`KismetMathLibrary.Normal` _returnvalue_3) (`self.GetActorForwardVector`)))) (`self.FrontFacingMaxAngle`))
                  (bind (_outhit _returnvalue_8) (`KismetSystemLibrary.LineTraceSingle` _returnvalue_2 _returnvalue "TraceTypeQuery1" false (`|MakeArray` (`self.VRPawn`) :!type "Actor Object Reference") "None" true (struct :`R` 1.0 :`A` 1.0) (struct :`G` 1.0 :`A` 1.0) 1.0))
                  (if _returnvalue_8
                    (if _lookedat :!label _label
                      (set `self.LookedAt` false)
                      (`self.LookEnded` self self (`self.VRPawn`)))
                    (elif _returnvalue_5
                      (`|ExecutionSequence`
                        (:`then_0`
                          (if (<= _returnvalue_7 _returnvalue_6)
                            (if (not _lookedat)
                              (set `self.LookedAt` true)
                              (`self.LookStarted` self self (`self.VRPawn`)))
                            (else
                              (goto _label))))
                        (:`then_1`
                          (if (`self.DrawLookPoint`)
                            (`ActorComponent.SetActive` (`self.LookPoint`) (<= _returnvalue_7 (* _returnvalue_6 4.0)) false))))))
                  (else
                    (goto _label)))
                (else
                  (goto _label))))))))))

(fn `IsLookedAt`
  (returns (LookedAt :type Boolean))
  (return (`self.LookedAt`)))

(fn `UserConstructionScript`
  (set `self.MaxLookDistanceSq` (`KismetMathLibrary.Square` (`self.LookPrecisionFactor`)))
  (set `self.MaxPlayerDistanceSq` (`KismetMathLibrary.Square` (`self.MaxPlayerDistance`)))
  (`SceneComponent.SetVisibility` (`self.LookPoint`) (`self.DrawLookPoint`) false))