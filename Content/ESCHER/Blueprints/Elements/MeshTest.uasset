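; MeshTest is a test actor that animates a tapering, twisting stack of instanced plates.
; BeginPlay adds twenty blank instances to the Plates component.
; Every Tick rewrites the transforms from index 1 upward, spacing plates evenly in height and shrinking their footprint geometrically.
; Accumulated time drives a sine-plus-cosine yaw that grows with index, so higher plates swing further.
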(event `self.ReceiveBeginPlay`
  (for _ (range 1 21)
    (`InstancedStaticMeshComponent.AddInstance` (`self.Plates`) (`/Game/ESCHER/Blueprints/Core/BasicMacros.BlankTransform`))))

(event `self.ReceiveTick`
  (params (DeltaSeconds :type "Float (single-precision)"))
  (bind _time (`self.Time`))
  (`/Game/ESCHER/Blueprints/Core/BasicMacros.IncrementFloatBy` _time DeltaSeconds
    (:`  `
      (for _index (range 20)
        (bind _returnvalue (+ _index 1))
        (bind _returnvalue_2 (* (`KismetMathLibrary.MultiplyMultiply_FloatFloat` 0.8 (`KismetMathLibrary.Conv_IntToDouble` _returnvalue)) 3.6))
        (`InstancedStaticMeshComponent.UpdateInstanceTransform` (`self.Plates`) _returnvalue (`KismetMathLibrary.MakeTransform` (`KismetMathLibrary.MakeVector` 0.0 0.0 (* _returnvalue 35.0)) (`KismetMathLibrary.MakeRotator` 0.0 0.0 (+ (* _returnvalue 5.0) (* (* _returnvalue (`self.Time`)) (+ (`KismetMathLibrary.DegSin` (* _time 4.13)) (`KismetMathLibrary.DegCos` (* _time 6.12)))))) (`KismetMathLibrary.MakeVector` _returnvalue_2 _returnvalue_2 0.1)) false true false)))))

(fn `UserConstructionScript`)