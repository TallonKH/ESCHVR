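; Proxy actor that positions a controlled actor or component, mapping it across a linked portal's two ports while one is active.
; Each tick or manual update, it re-parents its own transform between PortA and PortB by the entered side, applies an initial offset, and moves the target and a sphere.
; Teleport sets or clears the single active portal.
; A non-zero ParentCancel bypasses remapping; the child-propagation logic for it is unwired.
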(event `self.ReceiveTick`
  (params (DeltaSeconds :type "Float (single-precision)"))
  (bind _returnvalue (`self.GetTransform`))
  (bind _initialoffset (`self.InitialOffset`))
  (bind _portalside (`self.PortalSide`))
  (bind _activeportal (`self.ActivePortal`))
  (bind _returnvalue_2 (`SceneComponent.K2_GetComponentToWorld` (`/Game/ESCHER/Blueprints/Elements/InvisPortal.PortA` _activeportal)))
  (bind _returnvalue_3 (`SceneComponent.K2_GetComponentToWorld` (`/Game/ESCHER/Blueprints/Elements/InvisPortal.PortB` _activeportal)))
  (bind _out (`/Game/ESCHER/Blueprints/Core/BasicMacros.ReParentTransform` (`self.GetTransform`) (`KismetMathLibrary.SelectTransform` _returnvalue_3 _returnvalue_2 _portalside) (`KismetMathLibrary.SelectTransform` _returnvalue_2 _returnvalue_3 _portalside)))
  (if (`self.AutoUpdate`)
    (`|ExecutionSequence` :!label _label
      (:`then_0`
        (`/Engine/EditorBlueprintResources/StandardMacros.IsValid` (`self.ActivePortal`)
          (:`Is Valid`
            (if (== (`self.ParentCancel`) 0) :!label _label_2
              (set `self.OffsetProxyTransform` (`KismetMathLibrary.ComposeTransforms` _initialoffset _out))
              (set `self.ProxyTransform` _out)
              (else
                (set `self.OffsetProxyTransform` (`KismetMathLibrary.ComposeTransforms` _initialoffset _returnvalue) :!label _label_3)
                (set `self.ProxyTransform` _returnvalue))))
          (:`Is Not Valid`
            (goto _label_3))))
      (:`then_1`
        (`SceneComponent.K2_SetWorldTransform` (`self.Sphere`) (`self.OffsetProxyTransform`) false false)
        (if (`self.UseActor`)
          (`self.K2_SetActorTransform` (`self.ControlledActor`) (`self.OffsetProxyTransform`) false false)
          (else
            (`SceneComponent.K2_SetWorldTransform` (`self.ControlledComponent`) (`self.OffsetProxyTransform`) false false)))))))

(event `ManualUpdate`
  (goto _label))

(event `/Game/ESCHER/Blueprints/Core/Portalable.Teleport`
  (params (Portal :type "/Game/ESCHER/Blueprints/Elements/InvisPortal Object Reference") (side :type Boolean) (From :type "Transform Structure") (To :type "Transform Structure"))
  (bind _activeportal (`self.ActivePortal`))
  (`/Engine/EditorBlueprintResources/StandardMacros.IsValid` _activeportal
    (:`Is Valid`
      (if (== Portal _activeportal)
        (if (xor side (`self.PortalSide`))
          (set `self.ActivePortal` null)
          (goto _label_3)
          (else
            (`KismetSystemLibrary.PrintString` "!!! PROXY ENTERED SAME PORTAL MULTIPLE TIMES !!!" true true (struct :`R` 1.0 :`G` 0.006772 :`A` 1.0) 25.0)))
        (else
          (`KismetSystemLibrary.PrintString` "!!! PROXY COMPONENT CANNOT HANDLE MULTIPLE PORTALS !!!" true true (struct :`R` 1.0 :`G` 0.006772 :`A` 1.0) 25.0))))
    (:`Is Not Valid`
      (set `self.ActivePortal` Portal)
      (set `self.PortalSide` side)
      (goto _label_2))))

(fn `Calibrate`)

(fn `Get Origin`
  (returns (Origin :type "Vector Structure"))
  (return (.location (`self.OffsetProxyTransform`))))

(fn `UserConstructionScript`
  (set `self.ProxyTransform` (`self.GetTransform`)))