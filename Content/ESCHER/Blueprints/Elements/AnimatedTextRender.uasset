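; AnimatedTextRender is a world text actor with a typewriter reveal, driven by Erased, Writing, Written and Erasing states.
; The construction script styles the text, previews the initial state, draws a DisplayWidth guide line and sizes a timeline from per-character delays.
; While writing, timeline updates append characters as playback passes each threshold, with custom delays looked up by character code.
; Erasing reverses the timeline, but the update loop only advances the character index.
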(event `self.ReceiveBeginPlay`
  (`self.SetAnimationState` (`self.InitialState`)))

(event `SetAnimationState`
  (params (State :type "/Game/ESCHER/Blueprints/Core/TextAnimationState Enum" :default "NewEnumerator0"))
  (bind _resulttextasstring (`self.ResultTextAsString`))
  (bind _nextchunktime (`self.NextChunkTime`))
  (bind _currentcharindex (`self.CurrentCharIndex`))
  (bind _animation (`self.Animation`))
  (bind (_value _returnvalue) (`BlueprintMapLibrary.Map_Find` (`self.DelayMultipliersChars`) (`KismetStringLibrary.GetCharacterAsNumber` _resulttextasstring (- _currentcharindex 1))))
  (switch `/Game/ESCHER/Blueprints/Core/TextAnimationState` State
    (:`NewEnumerator0`
      (`TimelineComponent.SetNewTime` _animation 0.0))
    (:`NewEnumerator1`
      (`Timeline|Animation` :!label _label
        (:`Update`
          (while (>= (`TimelineComponent.GetPlaybackPosition` _animation) (`self.NextChunkTime`))
            (`TextRenderComponent.K2_SetText` (`self.FullText`) (`KismetTextLibrary.Conv_StringToText` (`KismetStringLibrary.GetSubstring` _resulttextasstring 0 _currentcharindex)))
            (`/Engine/EditorBlueprintResources/StandardMacros.IncrementInt` (`self.CurrentCharIndex`)
              (:`  `
                (if _returnvalue
                  (`/Game/ESCHER/Blueprints/Core/BasicMacros.IncrementFloatBy` _nextchunktime (* (`self.AnimationSpeed`) _value))
                  (else
                    (`/Game/ESCHER/Blueprints/Core/BasicMacros.IncrementFloatBy` _nextchunktime (* (`self.LetterDelay`) (`self.AnimationSpeed`)))))))))))
    (:`NewEnumerator2`
      (`TimelineComponent.SetNewTime` _animation 1.0))
    (:`NewEnumerator3`
      (goto _label :!via `Reverse`))))

(fn `SetTextRenderParams`
  (params (TextRenderComponent :type "TextRenderComponent Object Reference"))
  (`PrimitiveComponent.SetMaterial` TextRenderComponent 0 (`self.Material`))
  (`TextRenderComponent.SetFont` TextRenderComponent (`self.Font`))
  (`TextRenderComponent.SetWorldSize` TextRenderComponent (`self.TextSize`))
  (`TextRenderComponent.SetXScale` TextRenderComponent (`self.XScale`))
  (`TextRenderComponent.SetYScale` TextRenderComponent (`self.YScale`))
  (`TextRenderComponent.SetHorizSpacingAdjust` TextRenderComponent (`self.XSpacing`))
  (`TextRenderComponent.SetVertSpacingAdjust` TextRenderComponent (`self.YSpacing`))
  (`TextRenderComponent.SetHorizontalAlignment` TextRenderComponent (`self.HorizontalAlignement`))
  (`TextRenderComponent.SetVerticalAlignment` TextRenderComponent (`self.VerticalAlignment`)))

(fn `UserConstructionScript`
  (bind _fulltext (`self.FullText`))
  (bind _animationlength (`self.AnimationLength`))
  (bind _customdelays (`self.CustomDelays`))
  (bind _fulltext_2 (`self.FullText`))
  (bind _returnvalue (`SceneComponent.K2_GetComponentLocation` _fulltext_2))
  (`|ExecutionSequence`
    (:`then_1`
      (`self.SetTextRenderParams` (`self.FullText`)))
    (:`then_2`
      (set `self.ResultTextAsString` (`KismetTextLibrary.Conv_TextToString` (`self.ResultText`))))
    (:`then_3`
      (`KismetSystemLibrary.DrawDebugLine` _returnvalue (+ _returnvalue (* (`SceneComponent.GetRightVector` _fulltext_2) (* -1 (`self.DisplayWidth`)))) (struct :`R` 1.0 :`G` 1.0 :`B` 1.0 :`A` 1.0) 0.1 2.0))
    (:`then_4`
      (`BlueprintMapLibrary.Map_Clear` (`self.DelayMultipliersChars`))
      (bind _keys (`BlueprintMapLibrary.Map_Keys` _customdelays))
      (for _array_element _keys
        (`BlueprintMapLibrary.Map_Add` (`self.DelayMultipliersChars`) (`KismetStringLibrary.GetCharacterAsNumber` _array_element) (`BlueprintMapLibrary.Map_Find` _customdelays _array_element))))
    (:`then_5`
      (set `self.AnimationLength` 0.0)
      (for _index (range (`KismetStringLibrary.Len` (`self.ResultTextAsString`)))
        (bind (_value _returnvalue_2) (`BlueprintMapLibrary.Map_Find` (`self.DelayMultipliersChars`) (`KismetStringLibrary.GetCharacterAsNumber` (`self.ResultTextAsString`) _index)))
        (if _returnvalue_2
          (`/Game/ESCHER/Blueprints/Core/BasicMacros.IncrementFloatBy` _animationlength _value)
          (else
            (`/Game/ESCHER/Blueprints/Core/BasicMacros.IncrementFloatBy` _animationlength (`self.LetterDelay`)))))
      (bind _returnvalue_3 (`/Game/ESCHER/Blueprints/Core/BasicMacros.MultiplyFloatBy` (`self.AnimationLength`) (`self.AnimationSpeed`))
        (:`  `
          (`TimelineComponent.SetTimelineLength` (`self.Animation`) _returnvalue_3))))
    (:`then_6`
      (switch `/Game/ESCHER/Blueprints/Core/TextAnimationState` (`self.InitialState`)
        (:`NewEnumerator0`
          (`TextRenderComponent.K2_SetText` _fulltext (`/Game/ESCHER/Blueprints/Core/BasicMacros.BlankText`) :!label _label))
        (:`NewEnumerator1`
          (goto _label))
        (:`NewEnumerator2`
          (`TextRenderComponent.K2_SetText` _fulltext (`self.ResultText`) :!label _label_2)
          (`TimelineComponent.SetNewTime` (`self.Animation`) (`self.AnimationLength`)))
        (:`NewEnumerator3`
          (goto _label_2))))))