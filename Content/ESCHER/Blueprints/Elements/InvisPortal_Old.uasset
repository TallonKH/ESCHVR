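; Portal actor linking PortA and PortB, carrying physics objects and rays between them.
; Overlapping PhysObjs get GhostObj clones, which Tick mirrors through the opposite portal, swapping body and ghost with re-oriented velocity when the origin crosses.
; Burst and persistent rays continue from the other portal by re-parenting transforms, with burst hits re-broadcast as ghosts.
; Scene-capture view code and part of object registration, including side tracking, are disconnected.
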(event `self.ReceiveBeginPlay`
  (bind _initialtracked (`self.InitialTracked`))
  (`|ExecutionSequence`
    (:`then_0`
      (bind _keys (`BlueprintMapLibrary.Map_Keys` _initialtracked))
      (for _array_element _keys
        (`self.RegisterPhysObj` _array_element (`BlueprintMapLibrary.Map_Find` _initialtracked _array_element))))))

(event `self.ReceiveTick`
  (params (DeltaSeconds :type "Float (single-precision)"))
  (bind _portb (`self.PortB`))
  (bind _porta (`self.PortA`))
  (bind _portb_2 (`self.PortB`))
  (bind _porta_2 (`self.PortA`))
  (bind _tickdelay (`self.TickDelay`))
  (bind _ticker (`self.Ticker`))
  (bind _returnvalue (`/Game/ESCHER/Blueprints/Core/BasicMacros.IncrementFloatBy` _ticker DeltaSeconds)
    (:`  `
      (if (>= _returnvalue _tickdelay)
        (set `self.Ticker` (mod _ticker _tickdelay))
        (`|ExecutionSequence`
          (:`then_0`
            (for (_array_element _array_index) (`self.TrackedPObjects`)
              (bind _output (`|GetArrayItem` (`self.TrackedObjSide`) _array_index))
              (`SceneComponent.K2_SetWorldTransform` (`/Game/ESCHER/Blueprints/Elements/GhostObj.GhostMesh` (`|GetArrayItem` (`self.Clones`) _array_index)) (`/Game/ESCHER/Blueprints/Core/BasicMacros.ReParentTransformNegative` (`SceneComponent.K2_GetComponentToWorld` (`/Game/ESCHER/Blueprints/Core/PhysObj.MainMesh` _array_element)) (`SceneComponent.K2_GetComponentToWorld` (select `bool` _output :`false` _porta_2 :`true` _portb :!type "SceneComponent Object Reference")) (`SceneComponent.K2_GetComponentToWorld` (select `bool` _output :`false` _portb :`true` _porta_2 :!type "SceneComponent Object Reference"))) false false)))
          (:`then_1`
            (for _array_element_2 (`self.TouchedPhysObjects`)
              (bind _value (`BlueprintMapLibrary.Map_Find` (`self.TrackedObjMap`) _array_element_2))
              (bind _output_2 (`|GetArrayItem` (`self.TrackedObjSide`) _value))
              ;[1 1 1] Origin of object has passed to Ghost side of portal
              (if (< (`KismetMathLibrary.Dot_VectorVector` (- (`SceneComponent.K2_GetComponentLocation` (`/Game/ESCHER/Blueprints/Core/PhysObj.MainMesh` _array_element_2)) (`KismetMathLibrary.SelectVector` (`SceneComponent.K2_GetComponentLocation` _portb_2) (`SceneComponent.K2_GetComponentLocation` _porta) _output_2)) (`KismetMathLibrary.SelectVector` (`KismetMathLibrary.NegateVector` (`SceneComponent.GetForwardVector` _portb_2)) (`SceneComponent.GetForwardVector` _porta) _output_2)) 0.0)
                (`self.SwapGhost` _value)))))))))

(event `self.PortA.OnComponentBeginOverlap`
  (params (OverlappedComponent :type "PrimitiveComponent Object Reference") (OtherActor :type "Actor Object Reference") (OtherComp :type "PrimitiveComponent Object Reference") (OtherBodyIndex :type Integer) (bFromSweep :type Boolean) (SweepResult :type "HitResult Structure (by ref)"))
  (`KismetSystemLibrary.PrintString` "Actor Hit A" true true (struct :`R` 1.0 :`G` 0.926854 :`A` 1.0) 90.0)
  (bind _asphys_obj (cast `/Game/ESCHER/Blueprints/Core/PhysObj` OtherActor))
  (`KismetArrayLibrary.Array_Add` (`self.TouchedPhysObjects`) _asphys_obj)
  (`self.RegisterPhysObj` _asphys_obj))

(event `self.PortA.OnComponentEndOverlap`
  (params (OverlappedComponent :type "PrimitiveComponent Object Reference") (OtherActor :type "Actor Object Reference") (OtherComp :type "PrimitiveComponent Object Reference") (OtherBodyIndex :type Integer))
  (`KismetSystemLibrary.PrintString` "Actor Unhit A" true true (struct :`G` 0.345177 :`B` 1.0 :`A` 1.0) 90.0)
  (bind _asphys_obj (cast `/Game/ESCHER/Blueprints/Core/PhysObj` OtherActor))
  (`KismetArrayLibrary.Array_RemoveItem` (`self.TouchedPhysObjects`) _asphys_obj))

(event `self.PortB.OnComponentBeginOverlap`
  (params (OverlappedComponent :type "PrimitiveComponent Object Reference") (OtherActor :type "Actor Object Reference") (OtherComp :type "PrimitiveComponent Object Reference") (OtherBodyIndex :type Integer) (bFromSweep :type Boolean) (SweepResult :type "HitResult Structure (by ref)"))
  (`KismetSystemLibrary.PrintString` "Actor Hit B" true true (struct :`R` 1.0 :`G` 0.926854 :`A` 1.0) 90.0)
  (bind _asphys_obj (cast `/Game/ESCHER/Blueprints/Core/PhysObj` OtherActor))
  (`KismetArrayLibrary.Array_Add` (`self.TouchedPhysObjects`) _asphys_obj)
  (`self.RegisterPhysObj` _asphys_obj true))

(event `self.PortB.OnComponentEndOverlap`
  (params (OverlappedComponent :type "PrimitiveComponent Object Reference") (OtherActor :type "Actor Object Reference") (OtherComp :type "PrimitiveComponent Object Reference") (OtherBodyIndex :type Integer))
  (`KismetSystemLibrary.PrintString` "Actor Unhit B" true true (struct :`G` 0.237268 :`B` 1.0 :`A` 1.0) 90.0)
  (bind _asphys_obj (cast `/Game/ESCHER/Blueprints/Core/PhysObj` OtherActor))
  (`KismetArrayLibrary.Array_RemoveItem` (`self.TouchedPhysObjects`) _asphys_obj))

(event `TrackedBurstRayEvent`
  (params (Handler :type "/Game/ESCHER/Blueprints/Core/BurstRayHandler Object Reference") (Side :type Boolean) (SegmentID :type Integer))
  (`|ExecutionSequence`
    (:`then_0`
      (`BlueprintMapLibrary.Map_Add` (`self.TrackedBurstRaySide`) SegmentID Side))
    (:`then_1`
      (add `/Game/ESCHER/Blueprints/Core/BurstRayHandler.OnRayBlocked` Handler (delegate `TrackedBurstRayBlocked`)))
    (:`then_2`
      (add `/Game/ESCHER/Blueprints/Core/BurstRayHandler.OnRayPassed` Handler (delegate `TrackedBurstRayPassed`)))
    (:`then_3`
      (add `/Game/ESCHER/Blueprints/Core/BurstRayHandler.OnRayFinished` Handler (delegate `BurstRayFinished`)))))

(event `TrackedBurstRayBlocked`
  (params (Handler :type "/Game/ESCHER/Blueprints/Core/BurstRayHandler Object Reference") (SegmentID :type Integer) (Hit :type "HitResult Structure") (DoEffects :type Boolean) (Terminal :type Boolean) (Ghost :type Boolean))
  (bind (_bblockinghit _binitialoverlap _time _distance _location _impactpoint _normal _impactnormal _physmat _hitactor _hitcomponent _hitbonename _hititem _faceindex _tracestart _traceend) (`GameplayStatics.BreakHitResult` Hit))
  (bind _porta (`self.PortA`))
  (bind _portb (`self.PortB`))
  (bind _value (`BlueprintMapLibrary.Map_Find` (`self.TrackedBurstRaySide`) SegmentID))
  (bind _returnvalue (`SceneComponent.K2_GetComponentToWorld` (select `bool` _value :`false` _portb :`true` _porta :!type "SceneComponent Object Reference")))
  (bind _returnvalue_2 (`SceneComponent.K2_GetComponentToWorld` (select `bool` _value :`false` _porta :`true` _portb :!type "SceneComponent Object Reference")))
  (bind _out (`/Game/ESCHER/Blueprints/Core/BasicMacros.ReParentVector` _normal _returnvalue_2 _returnvalue))
  (bind _out_2 (`/Game/ESCHER/Blueprints/Core/BasicMacros.ReParentPositionNegative` _location _returnvalue_2 _returnvalue))
  (if (not Ghost)
    (`/Game/ESCHER/Blueprints/Core/BurstRayHandler.OnRayBlocked` Handler Handler SegmentID (`GameplayStatics.MakeHitResult` _bblockinghit _binitialoverlap _time _distance _out_2 _out_2 _out _out _physmat null null "None" 0 0 _tracestart _traceend) DoEffects Terminal true)))

(event `TrackedBurstRayPassed`
  (params (Handler :type "/Game/ESCHER/Blueprints/Core/BurstRayHandler Object Reference") (SegmentID :type Integer) (Hit :type "HitResult Structure") (DoEffects :type Boolean) (Ghost :type Boolean))
  (bind (_bblockinghit _binitialoverlap _time _distance _location _impactpoint _normal _impactnormal _physmat _hitactor _hitcomponent _hitbonename _hititem _faceindex _tracestart _traceend) (`GameplayStatics.BreakHitResult` Hit))
  (bind _portb (`self.PortB`))
  (bind _porta (`self.PortA`))
  (bind _value (`BlueprintMapLibrary.Map_Find` (`self.TrackedBurstRaySide`) SegmentID))
  (bind _returnvalue (`SceneComponent.K2_GetComponentToWorld` (select `bool` _value :`false` _porta :`true` _portb :!type "SceneComponent Object Reference")))
  (bind _returnvalue_2 (`SceneComponent.K2_GetComponentToWorld` (select `bool` _value :`false` _portb :`true` _porta :!type "SceneComponent Object Reference")))
  (bind _out (`/Game/ESCHER/Blueprints/Core/BasicMacros.ReParentPositionNegative` _location _returnvalue _returnvalue_2))
  (bind _out_2 (`/Game/ESCHER/Blueprints/Core/BasicMacros.ReParentVector` _normal _returnvalue _returnvalue_2))
  (if (not Ghost)
    (`/Game/ESCHER/Blueprints/Core/BurstRayHandler.OnRayPassed` Handler Handler SegmentID (`GameplayStatics.MakeHitResult` _bblockinghit _binitialoverlap _time _distance _out _out _out_2 _out_2 _physmat null null "None" 0 0 _tracestart _traceend) DoEffects true)))

(event `BurstRayFinished`
  (params (Handler :type "/Game/ESCHER/Blueprints/Core/BurstRayHandler Object Reference") (SegmentIDs :type "Array of Integer (by ref)"))
  (for _array_element SegmentIDs
    (`BlueprintMapLibrary.Map_Remove` (`self.TrackedBurstRaySide`) _array_element))
  (remove `/Game/ESCHER/Blueprints/Core/BurstRayHandler.OnRayFinished` Handler (delegate `BurstRayFinished`))
  (remove `/Game/ESCHER/Blueprints/Core/BurstRayHandler.OnRayBlocked` Handler (delegate `TrackedBurstRayBlocked`))
  (remove `/Game/ESCHER/Blueprints/Core/BurstRayHandler.OnRayPassed` Handler (delegate `TrackedBurstRayPassed`)))

(event `BindUpdater`
  (params (Handler :type "/Game/ESCHER/Blueprints/Core/PersistentRayHandler Object Reference") (Segment :type "/Game/ESCHER/Blueprints/Core/PersistentRaySegment Object Reference"))
  (bind _prayhandlersegmentsmap (`self.PRayHandlerSegmentsMap`))
  (bind _handlerid (`/Game/ESCHER/Blueprints/Core/PersistentRayHandler.HandlerID` Handler))
  (bind (_value _returnvalue) (`BlueprintMapLibrary.Map_Find` (`self.PRayHandlerSegmentsMap`) _handlerid))
  (`|ExecutionSequence`
    (:`then_0`
      (if _returnvalue
        (set `self.PStructSetHolder` (`.Segments_10_56C20AD840214EC23A873D86101D5436` (break `/Game/ESCHER/Blueprints/Core/SegmentSet` _value)))
        (`BlueprintSetLibrary.Set_Add` (`self.PStructSetHolder`) Segment)
        (`BlueprintMapLibrary.Map_Remove` _prayhandlersegmentsmap _handlerid)
        (`BlueprintMapLibrary.Map_Add` _prayhandlersegmentsmap _handlerid (make `/Game/ESCHER/Blueprints/Core/SegmentSet` (`self.PStructSetHolder`)))
        (else
          (bind _output_get (set `self.PStructSetHolder` (`|MakeSet` Segment)))
          (`BlueprintMapLibrary.Map_Add` (`self.PRayHandlerSegmentsMap`) _handlerid (make `/Game/ESCHER/Blueprints/Core/SegmentSet` _output_get)))))
    (:`then_1`
      (add `/Game/ESCHER/Blueprints/Core/PersistentRayHandler.OnRayUpdated` Handler (delegate `RayUpdated`)))))

(event `RayUpdated`
  (params (Handler :type "/Game/ESCHER/Blueprints/Core/PersistentRayHandler Object Reference"))
  (bind _temp_prpassedside (`self.Temp_PRPassedSide`))
  (bind _porta (`self.PortA`))
  (bind _portb (`self.PortB`))
  (bind _returnvalue (`SceneComponent.K2_GetComponentToWorld` (select `bool` _temp_prpassedside :`false` _portb :`true` _porta :!type "SceneComponent Object Reference")))
  (bind _returnvalue_2 (`SceneComponent.K2_GetComponentToWorld` (select `bool` _temp_prpassedside :`false` _porta :`true` _portb :!type "SceneComponent Object Reference")))
  (bind _output_get (set `self.PStructSetHolder` (`.Segments_10_56C20AD840214EC23A873D86101D5436` (break `/Game/ESCHER/Blueprints/Core/SegmentSet` (`BlueprintMapLibrary.Map_Find` (`self.PRayHandlerSegmentsMap`) (`/Game/ESCHER/Blueprints/Core/PersistentRayHandler.HandlerID` Handler))))))
  (bind _result (`BlueprintSetLibrary.Set_ToArray` _output_get))
  (for _array_element _result
    (set `self.Temp_PRPassedSide` (`BlueprintMapLibrary.Map_Find` (`self.TrackedPersistentRaySide`) _array_element))
    (bind _value (`BlueprintMapLibrary.Map_Find` (`self.PersistentRays`) _array_element))
    (set `/Game/ESCHER/Blueprints/Core/PersistentRaySegment.SourceLocation` (`/Game/ESCHER/Blueprints/Core/BasicMacros.ReParentPositionNegative` (`/Game/ESCHER/Blueprints/Core/PersistentRaySegment.SourceLocation` _array_element) _returnvalue_2 _returnvalue) _value)
    (set `/Game/ESCHER/Blueprints/Core/PersistentRaySegment.Towards` (`/Game/ESCHER/Blueprints/Core/BasicMacros.ReParentVector` (`/Game/ESCHER/Blueprints/Core/PersistentRaySegment.Towards` _array_element) _returnvalue_2 _returnvalue) _value)
    (set `/Game/ESCHER/Blueprints/Core/PersistentRaySegment.Distance` (`/Game/ESCHER/Blueprints/Core/PersistentRaySegment.Distance` _array_element) _value)
    (set `/Game/ESCHER/Blueprints/Core/PersistentRaySegment.AccumulatedDistance` (`/Game/ESCHER/Blueprints/Core/PersistentRaySegment.AccumulatedDistance` _array_element) _value)))

(event `/Game/ESCHER/Blueprints/Core/PersistentRayDetecting.EndedBlockPRay`
  (params (UnhitComponent :type "PrimitiveComponent Object Reference") (Segment :type "/Game/ESCHER/Blueprints/Core/PersistentRaySegment Object Reference") (RayHandler :type "/Game/ESCHER/Blueprints/Core/PersistentRayHandler Object Reference"))
  (bind _pstructsetholder (`self.PStructSetHolder`))
  (bind _handlerid (`/Game/ESCHER/Blueprints/Core/PersistentRayHandler.HandlerID` RayHandler))
  (bind _persistentrays (`self.PersistentRays`))
  (bind _prayhandlersegmentsmap (`self.PRayHandlerSegmentsMap`))
  (`|ExecutionSequence`
    (:`then_0`
      (`/Game/ESCHER/Blueprints/Core/PersistentRaySegment.Destroy` (`BlueprintMapLibrary.Map_Find` _persistentrays Segment)))
    (:`then_1`
      (`BlueprintMapLibrary.Map_Remove` _persistentrays Segment)
      (set `self.PStructSetHolder` (`.Segments_10_56C20AD840214EC23A873D86101D5436` (break `/Game/ESCHER/Blueprints/Core/SegmentSet` (`BlueprintMapLibrary.Map_Find` (`self.PRayHandlerSegmentsMap`) (`/Game/ESCHER/Blueprints/Core/PersistentRayHandler.HandlerID` RayHandler)))))
      (`BlueprintSetLibrary.Set_Remove` _pstructsetholder Segment)
      (if (== (`BlueprintSetLibrary.Set_Length` _pstructsetholder) 0)
        (`BlueprintMapLibrary.Map_Remove` _prayhandlersegmentsmap _handlerid)
        (remove `/Game/ESCHER/Blueprints/Core/PersistentRayHandler.OnRayUpdated` RayHandler (delegate `RayUpdated`))
        (else
          (`BlueprintMapLibrary.Map_Remove` _prayhandlersegmentsmap _handlerid)
          (`BlueprintMapLibrary.Map_Add` _prayhandlersegmentsmap _handlerid (make `/Game/ESCHER/Blueprints/Core/SegmentSet` (`self.PStructSetHolder`))))))
    (:`then_3`
      (set `self.PStructSetHolder` (`|MakeSet`))
      (set `self.PRayHandlerSegmentsMap` (`self.PRayHandlerSegmentsMap`)))))

(fn `BeganBlockPRay`
  (params (Hit :type "HitResult Structure") (Segment :type "/Game/ESCHER/Blueprints/Core/PersistentRaySegment Object Reference") (RayHandler :type "/Game/ESCHER/Blueprints/Core/PersistentRayHandler Object Reference"))
  (returns (`Do Effects` :type Boolean) (Terminal :type Boolean))
  (return false false))

(fn `BeganPassPRay`
  (params (Hit :type "HitResult Structure") (Segment :type "/Game/ESCHER/Blueprints/Core/PersistentRaySegment Object Reference") (RayHandler :type "/Game/ESCHER/Blueprints/Core/PersistentRayHandler Object Reference"))
  (returns (DoEffects :type Boolean) (IsGhost :type Boolean))
  (locals (PassedSide :type Boolean))
  (bind _segment (`/Game/ESCHER/Blueprints/Core/PersistentRayHandler.CreateSegment` RayHandler Segment))
  (`BlueprintMapLibrary.Map_Add` (`self.PersistentRays`) Segment _segment)
  (`self.BindUpdater` RayHandler Segment)
  (`KismetArrayLibrary.Array_Add` (`/Game/ESCHER/Blueprints/Core/PersistentRaySegment.ActorsToIgnore` _segment) self)
  (return false true))

(fn `BlockedBRay`
  (params (Hit :type "HitResult Structure") (RayHandler :type "/Game/ESCHER/Blueprints/Core/BurstRayHandler Object Reference") (SegmentDepth :type Integer) (Direction :type "Vector Structure") (AccumulatedDistance :type "Float (double-precision)") (SegmentID :type Integer))
  (returns (DoEffects :type Boolean) (Terminal :type Boolean))
  (return false false))

(fn `PassedBRay`
  (params (Hit :type "HitResult Structure") (RayHandler :type "/Game/ESCHER/Blueprints/Core/BurstRayHandler Object Reference") (SegmentDepth :type Integer) (Direction :type "Vector Structure") (AccumulatedDistance :type "Float (double-precision)") (SegmentID :type Integer))
  (returns (DoEffects :type Boolean) (MakeGhost :type Boolean) (EndpointOverride :type "Vector Structure"))
  (locals (PassedSide :type Boolean))
  (bind (_bblockinghit _binitialoverlap _time _distance _location _impactpoint _normal _impactnormal _physmat _hitactor _hitcomponent _hitbonename _hititem _faceindex _tracestart) (`GameplayStatics.BreakHitResult` Hit))
  (bind _passedside (`local.PassedSide`))
  (bind _porta (`self.PortA`))
  (bind _portb (`self.PortB`))
  (bind _returnvalue (`SceneComponent.K2_GetComponentToWorld` (select `bool` _passedside :`false` _portb :`true` _porta :!type "SceneComponent Object Reference")))
  (bind _returnvalue_2 (`SceneComponent.K2_GetComponentToWorld` (select `bool` _passedside :`false` _porta :`true` _portb :!type "SceneComponent Object Reference")))
  (`|ExecutionSequence`
    (:`then_0`
      (if (== _hitcomponent (`self.PortA`))
        (set `local.PassedSide` true)
        (elif (not (== _hitcomponent (`self.PortB`)))
          (bind _asportal_trigger (cast `` _hitactor))
          (set `local.PassedSide` (`/Game/ESCHER/Blueprints/Elements/InvisPortal_Old.Side` _asportal_trigger)))))
    (:`then_1`
      (`self.TrackedBurstRayEvent` RayHandler (`local.PassedSide`) SegmentID))
    (:`then_2`
      (bind _endpoint (`/Game/ESCHER/Blueprints/Core/BurstRayHandler.SegmentFire` RayHandler (`/Game/ESCHER/Blueprints/Core/BasicMacros.ReParentPositionNegative` _tracestart _returnvalue_2 _returnvalue) (`/Game/ESCHER/Blueprints/Core/BasicMacros.ReParentVector` Direction _returnvalue_2 _returnvalue) (- (`/Game/ESCHER/Blueprints/Core/BurstRayHandler.MaxDistance` RayHandler) AccumulatedDistance) (+ SegmentDepth 1) AccumulatedDistance (`|MakeArray` self :!type "Actor Object Reference")))
      (return false true (`/Game/ESCHER/Blueprints/Core/BasicMacros.ReParentPositionNegative` _endpoint _returnvalue _returnvalue_2)))))

(fn `RegisterAPhysObj`
  (params (PhysObj :type "/Game/ESCHER/Blueprints/Core/PhysObj Object Reference (by ref)"))
  (`KismetSystemLibrary.PrintString` "Actor is PhysObj" true true (struct :`R` 0.412102 :`G` 1.0 :`A` 1.0) 90.0)
  (if (not (`BlueprintMapLibrary.Map_Contains` (`self.TrackedAObjects`) PhysObj))
    (bind _returnvalue (`|SpawnActorFromClass` "/Game/ESCHER/Blueprints/Elements/GhostObj.GhostObj_C" (`self.GetTransform` PhysObj) "Undefined" "OverrideRootScale" null null))))

(fn `RegisterPhysObj`
  (params (PhysObj :type "/Game/ESCHER/Blueprints/Core/PhysObj Object Reference (by ref)") (Side :type Boolean))
  (bind (_value _returnvalue) (`BlueprintMapLibrary.Map_Find` (`self.TrackedObjMap`) PhysObj))
  (`KismetSystemLibrary.PrintString` "Actor is PhysObj" true true (struct :`R` 0.412102 :`G` 1.0 :`A` 1.0) 90.0)
  (if _returnvalue
    (`KismetSystemLibrary.PrintString` "PhysObj is not new" true true (struct :`G` 1.0 :`B` 0.821918 :`A` 1.0) 90.0)
    (`KismetArrayLibrary.Array_Set` (`self.TrackedObjSide`) _value Side)
    (return)
    (else
      (`KismetSystemLibrary.PrintString` "PhysObj is new" true true (struct :`G` 1.0 :`B` 0.821918 :`A` 1.0) 90.0)
      (bind _returnvalue_2 (`KismetArrayLibrary.Array_Add` (`self.TrackedPObjects`) PhysObj))
      (`BlueprintMapLibrary.Map_Add` (`self.TrackedObjMap`) PhysObj _returnvalue_2)
      (bind _returnvalue_3 (`|SpawnActorFromClass` "/Game/ESCHER/Blueprints/Elements/GhostObj.GhostObj_C" (`self.GetTransform` PhysObj) "Undefined" "OverrideRootScale" null null))
      (`KismetArrayLibrary.Array_Add` (`self.Clones`) _returnvalue_3))))

(fn `SwapGhost`
  (params (Index :type Integer))
  (locals (Tfm :type "Transform Structure"))
  (bind _porta (`self.PortA`))
  (bind _portb (`self.PortB`))
  (bind _output (`|GetArrayItem` (`self.TrackedObjSide`) Index))
  (bind _ghostmesh (`/Game/ESCHER/Blueprints/Elements/GhostObj.GhostMesh` (`|GetArrayItem` (`self.Clones`) Index)))
  (bind _mainmesh (`/Game/ESCHER/Blueprints/Core/PhysObj.MainMesh` (`|GetArrayItem` (`self.TrackedPObjects`) Index)))
  (`/Game/ESCHER/Blueprints/Core/BasicMacros.SetNot` _output)
  (bind _returnvalue (`PrimitiveComponent.GetPhysicsLinearVelocity` _mainmesh "None"))
  (set `local.Tfm` (`SceneComponent.K2_GetComponentToWorld` _mainmesh))
  (`SceneComponent.K2_SetWorldTransform` _mainmesh (`SceneComponent.K2_GetComponentToWorld` _ghostmesh) false false)
  (`SceneComponent.K2_SetWorldTransform` _ghostmesh (`local.Tfm`) false false)
  (`PrimitiveComponent.SetPhysicsLinearVelocity` _mainmesh (`/Game/ESCHER/Blueprints/Core/BasicMacros.ReParentVector` _returnvalue (`SceneComponent.K2_GetComponentToWorld` (select `bool` _output :`false` _portb :`true` _porta :!type "SceneComponent Object Reference")) (`SceneComponent.K2_GetComponentToWorld` (select `bool` _output :`false` _porta :`true` _portb :!type "SceneComponent Object Reference"))) false "None")
  (return))

(fn `UnregisterAPhysObj`
  (params (Obj :type "/Game/ESCHER/Blueprints/Core/PhysObj Object Reference (by ref)"))
  (locals (Ghost :type "/Game/ESCHER/Blueprints/Elements/GhostObj Object Reference"))
  (bind _trackedaobjects (`self.TrackedAObjects`))
  (bind (_value _returnvalue) (`BlueprintMapLibrary.Map_Find` _trackedaobjects Obj))
  (set `local.Ghost` _value)
  (if _returnvalue
    (`BlueprintMapLibrary.Map_Remove` _trackedaobjects Obj)
    (`self.K2_DestroyActor` (`local.Ghost`))))

(fn `UnregisterPhysObj`
  (params (Key :type "/Game/ESCHER/Blueprints/Core/PhysObj Object Reference (by ref)"))
  (locals (Index :type Integer))
  (bind _trackedobjmap (`self.TrackedObjMap`))
  (bind _index (`local.Index`))
  (bind (_value _returnvalue) (`BlueprintMapLibrary.Map_Find` _trackedobjmap Key))
  (set `local.Index` _value)
  (if _returnvalue
    (`BlueprintMapLibrary.Map_Remove` _trackedobjmap Key)
    (`KismetArrayLibrary.Array_Remove` (`self.TrackedPObjects`) (`local.Index`))
    (`KismetArrayLibrary.Array_Remove` (`self.TrackedObjSide`) _index)
    (`self.K2_DestroyActor` (`|GetArrayItem` (`self.Clones`) _index))
    (`KismetArrayLibrary.Array_Remove` (`self.Clones`) (`local.Index`))
    (`KismetArrayLibrary.Array_RemoveItem` (`self.TouchedPhysObjects`) Key)))

(fn `UserConstructionScript`)