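; BurstRayHandler fires instant burst rays as traced segments, letting hit actors such as portals intervene.
; PrimaryFire resets results, fires the first segment and broadcasts completion.
; SegmentFire registers an ID and multi-line traces, querying BurstRayDetecting actors on blocks and passes; ghost hits override the endpoint for external handling.
; Passing handler, depth and accumulated distance allows chained segments, while events report each block, pass and segment.
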(event `self.ReceiveBeginPlay`
  (bind _outactors (`GameplayStatics.GetAllActorsOfClass` "/Game/ESCHER/Blueprints/Core/LevelVarHandler.LevelVarHandler_C"))
  (set `self.LevelVarHandler` (`|GetArrayItem` _outactors)))

(fn `PrimaryFire`
  (params (From :type "Vector Structure") (Torwards :type "Vector Structure") (ActorsToIgnore :type "Array of Actor Object Reference (by ref)"))
  (set `self.TerminalHits` (`|MakeArray`))
  (set `self.SegmentIDs` (`|MakeArray`))
  (`self.SegmentFire` From Torwards (`self.MaxDistance`) 0 0.0 ActorsToIgnore)
  (`self.OnRayFinished` self (`self.SegmentIDs`)))

(fn `SegmentFire`
  (params (From :type "Vector Structure") (Towards :type "Vector Structure") (Distance :type "Float (double-precision)") (SegmentDepth :type Integer) (AccumulatedDistance :type "Float (double-precision)") (ActorsToIgnore :type "Array of Actor Object Reference (by ref)"))
  (returns (Endpoint :type "Vector Structure"))
  (locals (EndLocation :type "Vector Structure") (CurrentHit :type "HitResult Structure") (SegmentID :type Integer))
  (bind _currenthit (`local.CurrentHit`))
  (bind _segmentid (`local.SegmentID`))
  (bind _segmentid_2 (`local.SegmentID`))
  (bind _currenthit_2 (`local.CurrentHit`))
  (`|ExecutionSequence`
    (:`then_0`
      (bind _id (`/Game/ESCHER/Blueprints/Core/LevelVarHandler.IncrementRayID` (`self.LevelVarHandler`)))
      (bind _output_get (set `local.SegmentID` _id))
      (`KismetArrayLibrary.Array_Add` (`self.SegmentIDs`) _output_get)
      (`/Engine/EditorBlueprintResources/StandardMacros.IncrementInt` (`self.ActiveSegments`)))
    (:`then_1`
      (bind _output_get_2 (set `local.EndLocation` (+ From (* Towards Distance))))
      (bind _outhits (`KismetSystemLibrary.LineTraceMulti` From _output_get_2 "TraceTypeQuery3" false ActorsToIgnore))
      (`|ExecutionSequence`
        (:`then_0`
          (for _array_element _outhits
            (set `local.CurrentHit` _array_element)
            (bind (_bblockinghit _binitialoverlap _time _distance _location _impactpoint _normal _impactnormal _physmat _hitactor) (`GameplayStatics.BreakHitResult` _array_element))
            (if _bblockinghit
              (`|ExecutionSequence`
                (:`then_0`
                  (bind _asburst_ray_detecting (cast `/Game/ESCHER/Blueprints/Core/BurstRayDetecting` _hitactor)
                    (:`then`
                      (bind _returnvalue (+ _distance AccumulatedDistance))
                      (bind (_doeffects _terminal) (`/Game/ESCHER/Blueprints/Core/BurstRayDetecting.BlockedBRay` _asburst_ray_detecting (`local.CurrentHit`) self SegmentDepth Towards _returnvalue (`local.SegmentID`)))
                      (`self.OnRayBlocked` self _segmentid_2 _currenthit _doeffects _terminal)
                      (if _terminal
                        (`KismetArrayLibrary.Array_Add` (`self.TerminalHits`) (`local.CurrentHit`))))
                    (:`CastFailed`
                      (`self.OnRayBlocked` self _segmentid_2 _currenthit true true)
                      (`KismetArrayLibrary.Array_Add` (`self.TerminalHits`) (`local.CurrentHit`)))))
                (:`then_1`
                  (set `local.EndLocation` _location)
                  (break)))
              (else
                (bind _asburst_ray_detecting_2 (cast `/Game/ESCHER/Blueprints/Core/BurstRayDetecting` _hitactor)
                  (:`then`
                    (bind (_doeffects_2 _makeghost _endpointoverride) (`/Game/ESCHER/Blueprints/Core/BurstRayDetecting.PassedBRay` _asburst_ray_detecting_2 (`local.CurrentHit`) self SegmentDepth Towards _returnvalue (`local.SegmentID`)))
                    (if _makeghost
                      (set `local.EndLocation` _endpointoverride)
                      (break)
                      (else
                        (`self.OnRayPassed` self _segmentid _currenthit_2 _doeffects_2))))
                  (:`CastFailed`
                    (`self.OnRayPassed` self _segmentid _currenthit_2 true)))))))
        (:`then_1`
          (`self.OnSegmentCreated` From (`local.EndLocation`) SegmentDepth))
        (:`then_2`
          (`/Engine/EditorBlueprintResources/StandardMacros.DecrementInt` (`self.ActiveSegments`)
            (:`  `
              (return (`local.EndLocation`)))))))))

(fn `UserConstructionScript`)