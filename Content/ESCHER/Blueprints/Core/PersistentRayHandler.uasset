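; PersistentRayHandler manages a continuous ray that starts and ends with primary fire, built from PersistentRaySegment objects linked to parent segments.
; Firing creates a root segment at maximum distance, Tick updates it while the ray is active, and ending fire destroys it.
; Segments are mapped by IDs from LevelVarHandler, with notifications on creation and update.
; It also provides a multi-hit line trace helper on a fixed trace channel.
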(event `self.ReceiveBeginPlay`
  (bind _outactors (`GameplayStatics.GetAllActorsOfClass` "/Game/ESCHER/Blueprints/Core/LevelVarHandler.LevelVarHandler_C"))
  (bind _output_get (set `self.LevelVarHandler` (`|GetArrayItem` _outactors)))
  (bind _id (`/Game/ESCHER/Blueprints/Core/LevelVarHandler.IncrementRayID` _output_get))
  (set `self.HandlerID` _id))

(event `self.ReceiveTick`
  (params (DeltaSeconds :type "Float (single-precision)"))
  (if (`self.RayActive`)
    (`/Game/ESCHER/Blueprints/Core/PersistentRaySegment.UpdateRay` (`self.RootSegment`))
    (`self.OnRayUpdated` self)))

(fn `CreateSegment`
  (params (Parent :type "/Game/ESCHER/Blueprints/Core/PersistentRaySegment Object Reference"))
  (returns (Segment :type "/Game/ESCHER/Blueprints/Core/PersistentRaySegment Object Reference"))
  (bind _id (`/Game/ESCHER/Blueprints/Core/LevelVarHandler.IncrementRayID` (`self.LevelVarHandler`)))
  (bind _returnvalue (`|GenericCreateObject` "/Game/ESCHER/Blueprints/Core/PersistentRaySegment.PersistentRaySegment_C" self Parent self _id))
  (`BlueprintMapLibrary.Map_Add` (`self.Segments`) (`/Game/ESCHER/Blueprints/Core/PersistentRaySegment.SegmentID` _returnvalue) _returnvalue)
  (`/Game/ESCHER/Blueprints/Core/PersistentRaySegment.Init` _returnvalue)
  (`self.OnSegmentCreated` self _returnvalue)
  (return _returnvalue))

(fn `DoLineTrace`
  (params (Start :type "Vector Structure") (End :type "Vector Structure") (ActorsToIgnore :type "Array of Actor Object Reference (by ref)"))
  (returns (OutHits :type "Array of HitResult Structure") (ReturnValue :type Boolean))
  (bind (_outhits _returnvalue) (`KismetSystemLibrary.LineTraceMulti` Start End "TraceTypeQuery3" false ActorsToIgnore))
  (return _outhits _returnvalue))

(fn `EndPrimaryFire`
  (if (`self.RayActive`)
    (`/Game/ESCHER/Blueprints/Core/PersistentRaySegment.Destroy` (`self.RootSegment`))))

(fn `PrimaryFireStart`
  (if (not (`self.RayActive`))
    (set `self.RayActive` true)
    (set `self.Segments` (`|MakeMap`))
    (bind _segment (`self.CreateSegment` null))
    (set `self.RootSegment` _segment)
    (set `/Game/ESCHER/Blueprints/Core/PersistentRaySegment.Distance` (`self.MaxDistance`) _segment)))

(fn `UserConstructionScript`)