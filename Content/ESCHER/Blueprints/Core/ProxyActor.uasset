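; Proxy actor that drives a controlled actor or component, plus a sphere, from its own transform, remapped through a portal when one is active.
; Each Tick it re-parents that transform between the portal's two ports, in a direction set by PortalSide, and composes it with InitialOffset.
; Teleport records the portal and side, and clears them on an opposite-side crossing of that portal.
; Only one portal is supported; invalid crossings print errors.
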(event `self.ReceiveTick`
  (params (DeltaSeconds :type "Float (single-precision)"))
  (bind _initialoffset (`self.InitialOffset`))
  (bind _portalside (`self.PortalSide`))
  (bind _activeportal (`self.ActivePortal`))
  (bind _returnvalue (`SceneComponent.K2_GetComponentToWorld` (`/Game/ESCHER/Blueprints/Elements/InvisPortal.PortA` _activeportal)))
  (bind _returnvalue_2 (`SceneComponent.K2_GetComponentToWorld` (`/Game/ESCHER/Blueprints/Elements/InvisPortal.PortB` _activeportal)))
  (`|ExecutionSequence`
    (:`then_0`
      (`/Engine/EditorBlueprintResources/StandardMacros.IsValid` (`self.ActivePortal`)
        (:`Is Valid`
          (set `self.ProxyTransform` (`KismetMathLibrary.ComposeTransforms` (`/Game/ESCHER/Blueprints/Core/BasicMacros.ReParentTransform` (`self.GetTransform`) (`KismetMathLibrary.SelectTransform` _returnvalue_2 _returnvalue _portalside) (`KismetMathLibrary.SelectTransform` _returnvalue _returnvalue_2 _portalside)) _initialoffset)))
        (:`Is Not Valid`
          (set `self.ProxyTransform` (`KismetMathLibrary.ComposeTransforms` (`self.GetTransform`) _initialoffset)))))
    (:`then_1`
      (`SceneComponent.K2_SetWorldTransform` (`self.Sphere`) (`self.ProxyTransform`) false false)
      (if (`self.UseActor`)
        (`self.K2_SetActorTransform` (`self.ControlledActor`) (`self.ProxyTransform`) false false)
        (else
          (`SceneComponent.K2_SetWorldTransform` (`self.ControlledComponent`) (`self.ProxyTransform`) false false))))))

(event `/Game/ESCHER/Blueprints/Core/Portalable.Teleport`
  (params (Portal :type "/Game/ESCHER/Blueprints/Elements/InvisPortal Object Reference") (side :type Boolean) (From :type "Transform Structure") (To :type "Transform Structure"))
  (bind _activeportal (`self.ActivePortal`))
  (`/Engine/EditorBlueprintResources/StandardMacros.IsValid` _activeportal
    (:`Is Valid`
      (if (== Portal _activeportal)
        (if (xor side (`self.PortalSide`))
          (set `self.ActivePortal` null)
          (else
            (`KismetSystemLibrary.PrintString` "!!! PROXY ENTERED SAME PORTAL MULTIPLE TIMES !!!" true true (struct :`R` 1.0 :`G` 0.006772 :`A` 1.0) 25.0)))
        (else
          (`KismetSystemLibrary.PrintString` "!!! PROXY COMPONENT CANNOT HANDLE MULTIPLE PORTALS !!!" true true (struct :`R` 1.0 :`G` 0.006772 :`A` 1.0) 25.0))))
    (:`Is Not Valid`
      (set `self.ActivePortal` Portal)
      (set `self.PortalSide` side))))

(fn `Calibrate`)

(fn `Get Origin`
  (returns (Origin :type "Vector Structure"))
  (return (.location (`self.ProxyTransform`))))

(fn `UserConstructionScript`)