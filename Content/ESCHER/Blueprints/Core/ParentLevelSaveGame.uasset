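; Parent level save game that stores the VR player's root location, surface normal and forward vector.
; WritePlayerData compares the VR pawn's current root values against the saved ones within a small tolerance.
; When any value differs, it overwrites all three and returns true; otherwise it returns false, signalling whether the saved data changed.
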(fn `WritePlayerData`
  (params (VRPawn :type "/Game/ESCHER/Blueprints/Elements/Player/VRPawn Object Reference"))
  (returns (Changed :type Boolean))
  (bind _rootlocation (`/Game/ESCHER/Blueprints/Elements/Player/VRPawn.RootLocation` VRPawn))
  (bind _rootnormal (`/Game/ESCHER/Blueprints/Elements/Player/VRPawn.RootNormal` VRPawn))
  (bind _returnvalue (`SceneComponent.GetForwardVector` (`/Game/ESCHER/Blueprints/Elements/Player/VRPawn.Root` VRPawn)))
  (if (or (!= (`self.PlayerLocation`) _rootlocation :`ErrorTolerance` 0.001) (!= (`self.PlayerNormal`) _rootnormal :`ErrorTolerance` 0.001) (!= (`self.PlayerForward`) _returnvalue :`ErrorTolerance` 0.001))
    (set `self.PlayerLocation` _rootlocation)
    (set `self.PlayerNormal` _rootnormal)
    (set `self.PlayerForward` _returnvalue)
    (return true)
    (else
      (return false))))